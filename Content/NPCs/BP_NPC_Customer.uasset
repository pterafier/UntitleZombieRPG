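; NPC customer that serves as the hand-in target for quests from BP_RandomQuestGenerator.
; A looping timer checks active state and quest stage to toggle a money-sign waypoint, while a faster timer updates its distance to the player in meters.
; Looking at an active customer enables a custom-depth highlight, cleared by timer once the player looks away.
; Interacting at the delivery stage ends the quest and deactivates the customer.
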(event `StartDistanceChecker`
  ;[0 0 0 1 74] Handle exclamation mark
  (bind _returnvalue (`KismetSystemLibrary.K2_SetTimerDelegate` (delegate `HandleMarker`) 2.0 true))
  (set `self.CheckDistanceTimer` _returnvalue))

(event `HandleMarker`
  ;[0 0 0 1 74] Handle exclamation mark
  (if (and (`self.isActiveCustomer`) (>= (`/Game/Blueprints/Quests/BP_RandomQuestGenerator.QuestStage` (`self.QuestGeneratorRef`)) 2))
    (set `self.PlayerInRange` true)
    (`|ExecutionSequence`
      (:`then_0`
        (`/Engine/EditorBlueprintResources/StandardMacros.DoOnce` false :!label _label
          (:`Completed`
            (`SceneComponent.SetHiddenInGame` (`self.MoneySignWidget`) false false)
            (`/Engine/EditorBlueprintResources/StandardMacros.DoOnce` false :!label _label_2
              (:`Completed`
                (bind _returnvalue (`KismetSystemLibrary.K2_SetTimerDelegate` (delegate `UpdateWidgetDistance`) 0.25 true))
                (set `self.WidgetDistanceTimerHandle` _returnvalue))))))
      (:`then_1`
        (goto _label_3 :!via `Reset`)))
    (else
      (set `self.PlayerInRange` false)
      (`|ExecutionSequence`
        (:`then_0`
          (`/Engine/EditorBlueprintResources/StandardMacros.DoOnce` false :!label _label_3
            (:`Completed`
              (`SceneComponent.SetHiddenInGame` (`self.MoneySignWidget`) true false)
              (if (`KismetSystemLibrary.K2_IsValidTimerHandle` (`self.WidgetDistanceTimerHandle`))
                (`KismetSystemLibrary.K2_ClearAndInvalidateTimerHandle` (`self.WidgetDistanceTimerHandle`))
                (goto _label_2 :!via `Reset`)
                (else
                  (goto _label_2 :!via `Reset`))))))
        (:`then_1`
          (goto _label :!via `Reset`))))))

(event `UpdateWidgetDistance`
  ;[0 0 0 1 74] Handle exclamation mark
  (set `TextBlock.Text` (`KismetTextLibrary.Conv_StringToText` (`KismetStringLibrary.Concat_StrStr` (`KismetTextLibrary.Conv_TextToString` (`KismetTextLibrary.Conv_IntToText` (`KismetMathLibrary.FTrunc` (/ (`KismetMathLibrary.Vector_Distance` (`self.K2_GetActorLocation`) (`self.K2_GetActorLocation` (`GameplayStatics.GetPlayerPawn` 0))) 100.0)))) " m")) (`/Game/UI/Common/Widgets/HUD/WB_Common_WaypointDashOrder.CommonTextBlock_151` (`self.As WB Common Waypoint Dash Order`))))

(event `self.ReceiveBeginPlay`
  (`parent.ReceiveBeginPlay`)
  (`self.SetReferences`)
  (`self.StartDistanceChecker`))

(event `/Game/Blueprints/Interfaces/BPI_Interact.LookAt`
  ;[0 0 0 1 50] Look at
  (if (`self.isActiveCustomer`)
    (`PrimitiveComponent.SetRenderCustomDepth` (`self.Mesh`) true)
    (bind _returnvalue (`KismetSystemLibrary.K2_SetTimerDelegate` (delegate `UnHighlightMesh`) (`GameplayStatics.GetWorldDeltaSeconds`) true))
    (set `self.UnhighlightTimerHandle` _returnvalue)
    (`/Engine/EditorBlueprintResources/StandardMacros.DoOnce` false
      (:`Completed`
        (`PrimitiveComponent.SetCustomDepthStencilValue` (`self.Mesh`) 250)))
    (else
      (`self.UnHighlightMesh`))))

(event `UnHighlightMesh`
  ;[0 0 0 1 50] Look at
  (if (not (== (`/Game/Player/Blueprints/BP_ThirdPersonCharacter.LookAtActor` (`self.Player Character Ref`)) self))
    (`PrimitiveComponent.SetRenderCustomDepth` (`self.Mesh`) false)
    (`KismetSystemLibrary.K2_ClearAndInvalidateTimerHandle` (`self.UnhighlightTimerHandle`))))

(event `SetCustomerActive`
  (set `self.isActiveCustomer` true))

(event `SetCustomerInactive`
  (set `self.isActiveCustomer` false)
  (`SceneComponent.SetHiddenInGame` (`self.MoneySignWidget`) true false))

(fn `Interact`
  (returns (ObjectiveID :type String))
  (if (== (`/Game/Blueprints/Quests/BP_RandomQuestGenerator.QuestStage` (`self.QuestGeneratorRef`)) 2)
    (`/Game/Blueprints/Quests/BP_RandomQuestGenerator.EndQuest` (`self.QuestGeneratorRef`))
    (`self.SetCustomerInactive`)
    (return "customer")))

(fn `SetReferences`
  (set `self.Player Character Ref` (`/Game/Blueprints/BFL_CommonFunctions.GetPlayerCharacterReference`))
  (bind _aswb_common_waypoint_dash_order (cast `/Game/UI/Common/Widgets/HUD/WB_Common_WaypointDashOrder` (`WidgetComponent.GetWidget` (`self.MoneySignWidget`))))
  (set `self.As WB Common Waypoint Dash Order` _aswb_common_waypoint_dash_order)
  (bind _returnvalue (`GameplayStatics.GetActorOfClass` "/Game/Blueprints/Quests/BP_RandomQuestGenerator.BP_RandomQuestGenerator_C"))
  (set `self.QuestGeneratorRef` _returnvalue))

(fn `UserConstructionScript`
  (`parent.UserConstructionScript`))