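; Base quest-giver NPC that shows or hides an exclamation-mark widget according to its quest state.
; A looping distance check starts a roughly per-frame timer while the player is in range, yawing the widget toward the player's camera and refreshing quest status and marker.
; Status comes from matching the NPC's ObjectiveID, or that ID suffixed with "1", against current-stage objectives in the player's quest log.
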(event `self.ReceiveBeginPlay`
  (set `self.Player Character Ref` (`/Game/Blueprints/BFL_CommonFunctions.GetPlayerCharacterReference`))
  (set `self.Player State Ref` (`/Game/Blueprints/BFL_CommonFunctions.GetPlayerStateReference`))
  (`KismetSystemLibrary.Delay` 0.2)
  (`self.UpdateQuestMarker`)
  (`self.StartDistanceChecker`))

(event `UpdateQuestMarker`
  (if (`self.PlayerInRange`)
    (switch `/Game/Blueprints/Quests/Data/E_QuestGiverState` (`self.State`)
      (:`NewEnumerator0`
        (`SceneComponent.SetHiddenInGame` (`self.Widget1`) false false :!label _label)
        (bind _aswb_exclamation_mark (cast `/Game/UI/WB_ExclamationMark` (`WidgetComponent.GetWidget` (`self.Widget1`))))
        (set `/Game/UI/WB_ExclamationMark.ExclamationMarkColor` (`self.Exclamation Mark Color`) _aswb_exclamation_mark)
        (`/Game/UI/WB_ExclamationMark.Update` _aswb_exclamation_mark))
      (:`NewEnumerator1`
        (goto _label))
      (:`NewEnumerator2`
        (`SceneComponent.SetHiddenInGame` (`self.Widget1`) true false :!label _label_2))
      (:`NewEnumerator3`
        (goto _label_2)))))

(event `StartDistanceChecker`
  (bind _returnvalue (`KismetSystemLibrary.K2_SetTimerDelegate` (delegate `CheckDistance`) 2.0 true))
  (set `self.CheckDistanceTimer` _returnvalue))

(event `CheckDistance`
  (if (<= (`self.GetDistanceTo` (`self.Player Character Ref`)) 8500.0)
    (set `self.PlayerInRange` true)
    (`/Engine/EditorBlueprintResources/StandardMacros.DoOnce` false :!label _label_3
      (:`Completed`
        (bind _returnvalue (`KismetSystemLibrary.K2_SetTimerDelegate` (delegate `SetWidgetRotation`) (`GameplayStatics.GetWorldDeltaSeconds`) true))
        (set `self.SetWidgetRotationTimer` _returnvalue)
        (`self.UpdateQuestMarker`)))
    (else
      (set `self.PlayerInRange` false)
      (`self.UpdateQuestMarker`)
      (if (`KismetSystemLibrary.K2_IsValidTimerHandle` (`self.SetWidgetRotationTimer`))
        (`KismetSystemLibrary.K2_ClearAndInvalidateTimerHandle` (`self.SetWidgetRotationTimer`))
        (goto _label_3 :!via `Reset`)
        (else
          (goto _label_3 :!via `Reset`))))))

(event `SetWidgetRotation`
  (bind (_returnvalue_roll _returnvalue_pitch _returnvalue_yaw) (`KismetMathLibrary.BreakRotator` (`KismetMathLibrary.FindLookAtRotation` (`SceneComponent.K2_GetComponentLocation` (`self.Widget1`)) (`SceneComponent.K2_GetComponentLocation` (`/Game/Player/Blueprints/BP_ThirdPersonCharacter.FollowCamera` (`self.Player Character Ref`))))))
  (`SceneComponent.K2_SetWorldRotation` (`self.Widget1`) (`KismetMathLibrary.MakeRotator` 0.0 0.0 _returnvalue_yaw) false false)
  (`self.CheckCurrentQuestStatus`)
  (`self.UpdateQuestMarker`))

(fn `CheckCurrentQuestStatus`
  (bind (_objectivename _objectivetype _objectiveid) (break `/Game/Blueprints/Quests/Data/Struct_Objectives` (`|GetArrayItem` (`.Objectives_61_82055BE24DF71941EA78CE8A46EE88C8` (break `/Game/Blueprints/Quests/Data/Struct_Quest` (`/Game/Blueprints/Quests/BP_QuestManager.QuestDetails` (`self.QuestManager`)))) (`/Game/Blueprints/Quests/BP_QuestManager.CurrentStage` (`self.QuestManager`)))))
  (for _array_element (`/Game/Blueprints/Quests/AC_QuestLogComponent.CurrentQuests` (`/Game/Player/Blueprints/BP_PlayerState.AC_QuestLogComponent` (`self.Player State Ref`))) :!label _label
    (for _array_element_2 (`.Objectives_61_82055BE24DF71941EA78CE8A46EE88C8` (break `/Game/Blueprints/Quests/Data/Struct_Quest` (`/Game/Blueprints/Quests/BP_QuestManager.QuestDetails` _array_element)))
      (if (`KismetStringLibrary.EqualEqual_StrStr` (`.ObjectiveID_17_96A1B54D496DCD2428B1F3BF4B281CA9` (break `/Game/Blueprints/Quests/Data/Struct_Objectives` _array_element_2)) (`self.Objective ID`))
        (set `self.QuestManager` _array_element)
        (goto _label :!via `Break`)))
    (`self.QuestManager`
      (:`then`
        (if (and (not (`KismetStringLibrary.EqualEqual_StrStr` _objectiveid (`self.Objective ID`))) (`self.hasBeenInteractedWith`))
          (set `self.State` "NewEnumerator3")
          (if (`KismetStringLibrary.EqualEqual_StrStr` _objectiveid (`KismetStringLibrary.Concat_StrStr` (`self.Objective ID`) (`KismetStringLibrary.Conv_IntToString` 1)))
            (set `self.State` "NewEnumerator1"))))
      (:`else`))))

(fn `UserConstructionScript`)