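; Interactable quest-giver NPC that highlights when looked at and returns objective IDs when interacted with.
; Lookat enables custom depth with a stencil value, and a looping frame-interval timer removes it once the player looks away.
; Interact switches on quest state, advancing from offering to awaiting, then completing when an incrementer-suffixed ObjectiveID matches a current-stage objective in the player's quest log.
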(event `self.ReceiveBeginPlay`
  (`parent.ReceiveBeginPlay`))

(event `/Game/Blueprints/Interfaces/BPI_Interact.LookAt`
  (`PrimitiveComponent.SetRenderCustomDepth` (`self.Mesh`) true)
  (bind _returnvalue (`KismetSystemLibrary.K2_SetTimerDelegate` (delegate `UnHighlightMesh`) (`GameplayStatics.GetWorldDeltaSeconds`) true))
  (set `self.UnhighlightTimerHandle` _returnvalue)
  (`/Engine/EditorBlueprintResources/StandardMacros.DoOnce` false
    (:`Completed`
      (`PrimitiveComponent.SetCustomDepthStencilValue` (`self.Mesh`) 250))))

(event `UnHighlightMesh`
  (if (not (== (`/Game/Player/Blueprints/BP_ThirdPersonCharacter.LookAtActor` (`self.Player Character Ref`)) self))
    (`PrimitiveComponent.SetRenderCustomDepth` (`self.Mesh`) false)
    (`KismetSystemLibrary.K2_ClearAndInvalidateTimerHandle` (`self.UnhighlightTimerHandle`))))

(fn `Interact`
  (returns (ObjectiveID :type String))
  (`KismetSystemLibrary.PrintString` (`KismetStringLibrary.Conv_IntToString` (`self.Incrementer`)))
  (switch `/Game/Blueprints/Quests/Data/E_QuestGiverState` (`self.State`)
    (:`NewEnumerator0`
      (set `self.State` "NewEnumerator3")
      (`/Engine/EditorBlueprintResources/StandardMacros.IncrementInt` (`self.Incrementer`)
        (:`  `
          (`self.CheckCurrentQuestStatus`)
          (set `self.hasBeenInteractedWith` true)
          (return (`self.Objective ID`)))))
    (:`NewEnumerator1`
      (set `self.Objective ID` (`KismetStringLibrary.Concat_StrStr` (`self.Objective ID`) (`KismetStringLibrary.Conv_IntToString` (`self.Incrementer`))))
      (`self.CheckCurrentQuestStatus`)
      (for _array_element (`/Game/Blueprints/Quests/AC_QuestLogComponent.CurrentQuests` (`/Game/Player/Blueprints/BP_PlayerState.AC_QuestLogComponent` (`self.Player State Ref`)))
        (if (`KismetStringLibrary.EqualEqual_StrStr` (`.ObjectiveID_17_96A1B54D496DCD2428B1F3BF4B281CA9` (break `/Game/Blueprints/Quests/Data/Struct_Objectives` (`|GetArrayItem` (`.Objectives_61_82055BE24DF71941EA78CE8A46EE88C8` (break `/Game/Blueprints/Quests/Data/Struct_Quest` (`/Game/Blueprints/Quests/BP_QuestManager.QuestDetails` _array_element))) (`/Game/Blueprints/Quests/BP_QuestManager.CurrentStage` _array_element)))) (`self.Objective ID`))
          (set `self.State` "NewEnumerator2")
          (`/Engine/EditorBlueprintResources/StandardMacros.IncrementInt` (`self.Incrementer`)
            (:`  `
              (return (`self.Objective ID`)))))))))

(fn `UserConstructionScript`
  (`parent.UserConstructionScript`))