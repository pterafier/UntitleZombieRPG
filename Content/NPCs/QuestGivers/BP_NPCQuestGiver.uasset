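; Quest-giver NPC that shows quest status with head-socket marker widgets and forwards Interact to ACQuestGiverComponent.
; Tick re-checks quest state every frame, showing the question mark, exclamation mark or neither, and yaws both toward the player's follow camera.
; Lookat highlights the mesh through custom depth stencil, with a looping timer clearing it once the player's LookAtActor changes.
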(event `UpdateQuestMarker`
  (`/Game/Blueprints/Quests/AC_QuestGiverComponent.CheckCurrentQuestStatus` (`self.AC_QuestGiverComponent`))
  (switch `/Game/Blueprints/Quests/Data/E_QuestGiverState` (`/Game/Blueprints/Quests/AC_QuestGiverComponent.QuestGiverState` (`self.AC_QuestGiverComponent`))
    (:`NewEnumerator0`
      (`SceneComponent.SetHiddenInGame` (`self.ExclamationMarkWidget`) true false)
      (`SceneComponent.SetHiddenInGame` (`self.QuestionMarkWidget`) false false))
    (:`NewEnumerator1`
      (`SceneComponent.SetHiddenInGame` (`self.ExclamationMarkWidget`) false false)
      (`SceneComponent.SetHiddenInGame` (`self.QuestionMarkWidget`) true false :!label _label))
    (:`NewEnumerator2`
      (`SceneComponent.SetHiddenInGame` (`self.ExclamationMarkWidget`) true false :!label _label_2)
      (goto _label))
    (:`NewEnumerator3`
      (goto _label_2))))

(event `self.ReceiveBeginPlay`
  (`parent.ReceiveBeginPlay`)
  (set `self.Player Character Ref` (`/Game/Blueprints/BFL_CommonFunctions.GetPlayerCharacterReference`))
  (`self.UpdateQuestMarker`))

(event `self.ReceiveTick`
  (params (DeltaSeconds :type "Float (single-precision)"))
  (bind (_returnvalue_roll _returnvalue_pitch _returnvalue_yaw) (`KismetMathLibrary.BreakRotator` (`KismetMathLibrary.FindLookAtRotation` (`SceneComponent.K2_GetComponentLocation` (`self.ExclamationMarkWidget`)) (`SceneComponent.K2_GetComponentLocation` (`/Game/Player/Blueprints/BP_ThirdPersonCharacter.FollowCamera` (`self.Player Character Ref`))))))
  (`parent.ReceiveTick` DeltaSeconds)
  (`SceneComponent.K2_SetWorldRotation` (`self.ExclamationMarkWidget`) (`KismetMathLibrary.MakeRotator` 0.0 0.0 _returnvalue_yaw) false false)
  (`SceneComponent.K2_SetWorldRotation` (`self.QuestionMarkWidget`) (`KismetMathLibrary.MakeRotator` 0.0 0.0 _returnvalue_yaw) false false)
  (`self.UpdateQuestMarker`))

(event `/Game/Blueprints/Interfaces/BPI_Interact.LookAt`
  (`PrimitiveComponent.SetRenderCustomDepth` (`self.Mesh`) true)
  (bind _returnvalue (`KismetSystemLibrary.K2_SetTimerDelegate` (delegate `UnHighlightMesh`) (`GameplayStatics.GetWorldDeltaSeconds`) true))
  (set `self.UnhighlightTimerHandle` _returnvalue)
  (`/Engine/EditorBlueprintResources/StandardMacros.DoOnce` false
    (:`Completed`
      (`PrimitiveComponent.SetCustomDepthStencilValue` (`self.Mesh`) 250))))

(event `UnHighlightMesh`
  (if (not (== (`/Game/Player/Blueprints/BP_ThirdPersonCharacter.LookAtActor` (`self.Player Character Ref`)) self))
    (`PrimitiveComponent.SetRenderCustomDepth` (`self.Mesh`) false)
    (`KismetSystemLibrary.K2_ClearAndInvalidateTimerHandle` (`self.UnhighlightTimerHandle`))))

(fn `Interact`
  (returns (ObjectiveID :type String))
  (bind _objectiveid (`/Game/Blueprints/Interfaces/BPI_Interact.Interact` (`self.AC_QuestGiverComponent`)))
  (return _objectiveid))

(fn `UserConstructionScript`
  (`parent.UserConstructionScript`)
  (`SceneComponent.K2_AttachToComponent` (`self.QuestionMarkWidget`) (`self.Mesh`) "headSocket" "KeepRelative" "KeepRelative" "KeepRelative" true)
  (`SceneComponent.K2_AttachToComponent` (`self.ExclamationMarkWidget`) (`self.Mesh`) "headSocket" "KeepRelative" "KeepRelative" "KeepRelative" true))