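; Base enemy AI controller that runs BT_EnemyBase and sets its blackboard state to Patrolling, Investigating or Attacking from AI Perception.
; Seeing the player starts an attack, while sound or damage triggers investigation, only when patrolling or investigating.
; A looping timer polls sight stimulus age to drop attacks into investigation, and another timer returns investigation to patrol.
; An arrival-check timer for investigation locations is defined but never started here.
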(event `StartInvestigationLocationTimer`
  ;[0 0 0 1 90] Timers
  ;;[0.05 0.05 0.05] If the AI hears something, this timer checks if it's reached the location that it heard the sound. Once that happens, allow it the opportunity to stop investigating
  (bind _returnvalue (`KismetSystemLibrary.K2_SetTimerDelegate` (delegate `StopInvestigating`) 0.1 true))
  (set `self.CheckInvestigationLocation_TimerHandle` _returnvalue))

(event `self.ReceivePossess`
  (params (PossessedPawn :type "Pawn Object Reference"))
  (`self.RunBehaviorTree` "/Game/NPCs/Enemies/AI/BT_EnemyBase.BT_EnemyBase")
  (`self.SetStatePassive`))

(event `self.AIPerception.OnPerceptionUpdated`
  (params (UpdatedActors :type "Array of Actor Object Reference (by ref)"))
  (`self.HandleUpdatedPerception` UpdatedActors))

(event `StopInvestigating`
  ;[0 0 0 1 90] Timers
  ;;[0.05 0.05 0.05] If the AI hears something, this timer checks if it's reached the location that it heard the sound. Once that happens, allow it the opportunity to stop investigating
  (if (== (`self.K2_GetActorLocation` (`self.K2_GetPawn`)) (`self.InvestigationLocation`) :`ErrorTolerance` 200.0)
    (`self.StartInvestigationTimer`)))

(event `StartInvestigationTimer`
  ;[0 0 0 1 90] Timers
  ;;[0.05 0.05 0.05] Handles investigation timers. Allows AI to exit investigation state and return to patrolling
  (bind _returnvalue (`KismetSystemLibrary.K2_SetTimerDelegate` (delegate `CheckInvestigationState`) 5.0))
  (set `self.Investigation_TimerHandle` _returnvalue)
  (`KismetSystemLibrary.K2_ClearAndInvalidateTimerHandle` (`self.CheckInvestigationLocation_TimerHandle`)))

(event `CheckInvestigationState`
  ;[0 0 0 1 90] Timers
  ;;[0.05 0.05 0.05] Handles investigation timers. Allows AI to exit investigation state and return to patrolling
  (bind _currentstate (`self.GetCurrentState`))
  (switch `/Game/NPCs/Enemies/Data/E_EnemyState` _currentstate
    (:`NewEnumerator0`
      _)
    (:`NewEnumerator1`
      (`self.SetStatePassive`))
    (:`NewEnumerator2`
      _)
    (:`NewEnumerator3`
      _)
    (:`NewEnumerator4`
      _))
  (`KismetSystemLibrary.K2_ClearAndInvalidateTimerHandle` (`self.Investigation_TimerHandle`)))

(event `StartChaseTimer`
  ;[0 0 0 1 90] Timers
  ;;[0.05 0.05 0.05] Handles chase timers. Allows AI to exit combat state and return to patrolling
  (bind _returnvalue (`KismetSystemLibrary.K2_SetTimerDelegate` (delegate `StopChasing`) 0.1 true))
  (set `self.StopChasing_TimerHandle` _returnvalue)
  (goto _label :!via `Reset`))

(event `StopChasing`
  ;[0 0 0 1 90] Timers
  ;;[0.05 0.05 0.05] Handles chase timers. Allows AI to exit combat state and return to patrolling
  (bind (_stimulus _age _successfully_sensed) (`self.GetVisualStimulusAge`))
  (if (and (>= _age 5.0) _successfully_sensed)
    (`/Engine/EditorBlueprintResources/StandardMacros.DoOnce` false :!label _label
      (:`Completed`
        (`self.StopAttacking`)))))

(fn `CanSenseActor`
  (params (Actor :type "Actor Object Reference") (Sense :type "/Game/NPCs/Enemies/Data/E_Senses Enum" :default "NewEnumerator0"))
  (returns (Sensed :type Boolean) (Stimulus :type "AIStimulus Structure"))
  (bind _info (`AIPerceptionComponent.GetActorsPerception` (`self.AIPerception`) Actor))
  (for _array_element (`.LastSensedStimuli` (break `ActorPerceptionBlueprintInfo` _info))
    (bind _returnvalue (`AIPerceptionSystem.GetSenseClassForStimulus` _array_element))
    (if (== _returnvalue (select `/Game/NPCs/Enemies/Data/E_Senses` (`local.Sense`) :`NewEnumerator1` "/Script/AIModule.AISense_Sight" :`NewEnumerator2` "/Script/AIModule.AISense_Hearing" :`NewEnumerator3` "/Script/AIModule.AISense_Damage" :!type "Object Class Reference"))
      (return (`.bSuccessfullySensed` (break `AIStimulus` _array_element)) _array_element))))

(fn `GetCurrentState`
  (returns (CurrentState :type "/Game/NPCs/Enemies/Data/E_EnemyState Enum"))
  (return (cast `/Game/NPCs/Enemies/Data/E_EnemyState` (`BlackboardComponent.GetValueAsEnum` (`self.Blackboard`) (`self.State_BB_Name`)))))

(fn `GetDamageStimulusAge`
  (returns (Stimulus :type "AIStimulus Structure") (Age :type "Float (single-precision)") (`Successfully Sensed` :type Boolean))
  (locals (DamageStimulus :type "AIStimulus Structure"))
  (bind (_sensed _stimulus) (`self.CanSenseActor` (`GameplayStatics.GetPlayerCharacter` 0) "NewEnumerator3"))
  (bind _output_get (set `self.Visual Stimulus` _stimulus))
  (bind (_age _expirationage _strength _stimuluslocation _receiverlocation _tag _bsuccessfullysensed) (break `AIStimulus` _output_get))
  (return _output_get _age _bsuccessfullysensed))

(fn `GetVisualStimulusAge`
  (returns (Stimulus :type "AIStimulus Structure") (Age :type "Float (single-precision)") (`Successfully Sensed` :type Boolean))
  (locals (DamageStimulus :type "AIStimulus Structure"))
  (bind (_sensed _stimulus) (`self.CanSenseActor` (`GameplayStatics.GetPlayerCharacter` 0) "NewEnumerator1"))
  (bind _output_get (set `self.Visual Stimulus` _stimulus))
  (bind (_age _expirationage _strength _stimuluslocation _receiverlocation _tag _bsuccessfullysensed) (break `AIStimulus` _output_get))
  (return _output_get _age _bsuccessfullysensed))

(fn `HandleSensedDamage`
  (params (Actor :type "Actor Object Reference"))
  (bind _currentstate (`self.GetCurrentState`))
  (switch `/Game/NPCs/Enemies/Data/E_EnemyState` _currentstate
    (:`NewEnumerator0`
      _)
    (:`NewEnumerator1`
      _))
  (`self.SetStateAsInvestigating` (`self.K2_GetActorLocation` (`local.Actor`)))
  (`self.StartInvestigationTimer`))

(fn `HandleSensedSight`
  (params (Actor :type "Actor Object Reference"))
  (if (== Actor (`GameplayStatics.GetPlayerCharacter` 0))
    (bind _currentstate (`self.GetCurrentState`))
    ;[0 0 0] If the AI was patrolling or investigating when it saw something, start chase
    (switch `/Game/NPCs/Enemies/Data/E_EnemyState` _currentstate
      (:`NewEnumerator0`
        _)
      (:`NewEnumerator1`
        _))
    (`self.SetStateAttacking` (`local.Actor`) (`self.K2_GetActorLocation` (`GameplayStatics.GetPlayerCharacter` 0)))
    (`self.StartChaseTimer`)))

(fn `HandleSensedSound`
  (params (Location :type "Vector Structure"))
  (bind _currentstate (`self.GetCurrentState`))
  (switch `/Game/NPCs/Enemies/Data/E_EnemyState` _currentstate
    (:`NewEnumerator0`
      _)
    (:`NewEnumerator1`
      _))
  (`self.SetStateAsInvestigating` (`local.Location`))
  (`self.StartInvestigationTimer`))

(fn `HandleUpdatedPerception`
  (params (UpdatedActors :type "Array of Actor Object Reference"))
  (locals (Actor :type "Actor Object Reference"))
  ;[0 0 0] For each actor perceived:
  (for _array_element UpdatedActors
    (set `local.Actor` _array_element)
    (`|ExecutionSequence`
      (:`then_0`
        ;[0 0 0] If the AI sees something, handle it
        (bind _sensed (`self.CanSenseActor` (`local.Actor`) "NewEnumerator1"))
        (if _sensed
          (`self.HandleSensedSight` (`local.Actor`))))
      (:`then_1`
        ;[0 0 0] If the AI hears something, handle it
        (bind (_sensed_2 _stimulus) (`self.CanSenseActor` (`local.Actor`) "NewEnumerator2"))
        (if _sensed_2
          (bind (_age _expirationage _strength _stimuluslocation) (break `AIStimulus` _stimulus))
          (set `self.InvestigationLocation` _stimuluslocation)
          (`self.HandleSensedSound` _stimuluslocation)))
      (:`then_2`
        ;[0 0 0] If the AI takes damage, handle it
        (bind _sensed_3 (`self.CanSenseActor` (`local.Actor`) "NewEnumerator3"))
        (if _sensed_3
          (`self.HandleSensedDamage` (`local.Actor`))))))
  (return))

(fn `SetStateAsInvestigating`
  (params (Location :type "Vector Structure"))
  (`BlackboardComponent.SetValueAsEnum` (`self.Blackboard`) (`self.State_BB_Name`) (enumliteral `/Game/NPCs/Enemies/Data/E_EnemyState` "NewEnumerator1"))
  (`BlackboardComponent.SetValueAsVector` (`self.Blackboard`) (`self.PointOfInterest_BB_Name`) (`local.Location`)))

(fn `SetStateAttacking`
  (params (AttackTarget :type "Actor Object Reference") (TargetLocation :type "Vector Structure"))
  (`BlackboardComponent.SetValueAsObject` (`self.Blackboard`) (`self.TargetActor_BB_Name`) AttackTarget)
  (`BlackboardComponent.SetValueAsEnum` (`self.Blackboard`) (`self.State_BB_Name`) (enumliteral `/Game/NPCs/Enemies/Data/E_EnemyState` "NewEnumerator3"))
  (`BlackboardComponent.SetValueAsVector` (`self.Blackboard`) (`self.LastKnownLocation_BB_Name`) (`local.TargetLocation`)))

(fn `SetStatePassive`
  (`BlackboardComponent.SetValueAsEnum` (`self.Blackboard`) (`self.State_BB_Name`) (enumliteral `/Game/NPCs/Enemies/Data/E_EnemyState` "NewEnumerator0")))

(fn `StopAttacking`
  (`BlackboardComponent.SetValueAsObject` (`self.Blackboard`) (`self.TargetActor_BB_Name`) null)
  (`self.SetStateAsInvestigating` (`self.K2_GetActorLocation` (`self.K2_GetPawn`)))
  (`KismetSystemLibrary.K2_ClearAndInvalidateTimerHandle` (`self.StopChasing_TimerHandle`))
  (`self.StartInvestigationTimer`))

(fn `UserConstructionScript`)