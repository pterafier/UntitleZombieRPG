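; Base zombie enemy that handles damage, hit reactions and death, with randomized walk and run speeds.
; Headshot damage types remove a helmet or multiply damage, then hits report to AI damage sense and reduce attribute-set health.
; Surviving hits play a montage and occasionally halt movement; death flags the Blackboard, ragdolls with an impulse, notifies the player's objective and destroys the actor.
; Effects, helmet, patrol and speed functions are empty stubs.
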(event `self.ReceiveBeginPlay`
  (add `self.OnTakeAnyDamage` (delegate `OnTakeAnyDamage_Event`))
  (set `self.PlayerRef` (`/Game/Blueprints/BFL_CommonFunctions.GetPlayerCharacterReference`))
  (set `self.PlayerStateRef` (`/Game/Blueprints/BFL_CommonFunctions.GetPlayerStateReference`))
  (set `self.MaxWalkingSpeed` (`KismetMathLibrary.RandomFloatInRange` 50.0 125.0))
  (set `self.MaxRunningSpeed` (`KismetMathLibrary.RandomFloatInRange` 200.0 400.0)))

(event `OnTakeAnyDamage_Event`
  (params (DamagedActor :type "Actor Object Reference") (Damage :type "Float (single-precision)") (DamageType :type "DamageType Object Reference") (InstigatedBy :type "Controller Object Reference") (DamageCauser :type "Actor Object Reference"))
  (set `self.Instigated By` InstigatedBy)
  ;[0 0 0] True if player hit a headshot
  (set `self.IncomingDamage` Damage)
  (if (== (`GameplayStatics.GetObjectClass` DamageType) "/Game/Blueprints/Weapons/DamageTypes/BP_HeadshotDamageType.BP_HeadshotDamageType_C")
    (if (`self.hasHelmet`)
      (`self.RemoveHelmet`)
      (else
        (set `self.IncomingDamage` (* (`self.IncomingDamage`) (`self.HeadshotDamageMultiplier`)))
        (`KismetSystemLibrary.PrintString` "Took headshot damage" true true (struct :`G` 0.66 :`B` 1.0 :`A` 1.0) 10.0))))
  (`/Engine/EditorBlueprintResources/StandardMacros.DoOnce` false :!label _label
    (:`Completed`
      (`AISense_Damage.ReportDamageEvent` self (`self.Instigated By`) (`self.IncomingDamage`) (`self.K2_GetActorLocation`))
      (`/Game/Blueprints/Components/AC_BaseAttributeSet.ReduceHealth` (`self.AC_BaseAttributeSet`) (`self.IncomingDamage`))
      (if (<= (`/Game/Blueprints/Components/AC_BaseAttributeSet.GetHealth` (`self.AC_BaseAttributeSet`)) 0.0)
        (`self.OnDeath`)
        (`KismetSystemLibrary.Delay` 5.0)
        (`self.K2_DestroyActor`)
        (else
          (`|PlayMontage` (`self.Mesh`) (`self.HitReactionMontage`) 2.0
            (:`then`
              (`self.PlayHitEffects`)
              ;[0 0 0] 1 in 10 chance the hit stops the zombie from moving
              (if (== (`KismetMathLibrary.RandomIntegerInRange` 1 10) 5)
                (`CharacterMovementComponent.SetMovementMode` (`self.CharacterMovement`) "MOVE_None" 0)
                (goto _label :!via `Reset`)
                (else
                  (goto _label :!via `Reset`))))
            (:`OnCompleted`
              _)
            (:`OnBlendOut`
              _)
            (:`OnInterrupted`
              _))
          ;[0 0 0] In case the movement got stopped, reset it so the zombie can move again
          (`CharacterMovementComponent.SetMovementMode` (`self.CharacterMovement`) "MOVE_Walking" 0))))))

(fn `GetPatrolRoute`
  (returns (PatrolRoute :type "/Game/Blueprints/BP_PatrolRoute Object Reference") (`UsePatrolRoute?` :type Boolean))
  (return null false))

(fn `OnDeath`
  (set `self.isDead` true)
  (`/Engine/EditorBlueprintResources/StandardMacros.DoOnce` false
    (:`Completed`
      (`SkeletalMeshComponent.SetAnimationMode` (`self.Mesh`) "AnimationCustomMode" true)
      (`BlackboardComponent.SetValueAsBool` (`AIController.Blackboard` (`AIBlueprintHelperLibrary.GetAIController` self)) (`self.isDead_BB_BoolName`) true)
      (`PrimitiveComponent.SetCollisionObjectType` (`self.Mesh`) "ECC_PhysicsBody")
      (`PrimitiveComponent.SetSimulatePhysics` (`self.Mesh`) true)
      (`PrimitiveComponent.SetCollisionResponseToChannel` (`self.CapsuleComponent`) "ECC_Pawn" "ECR_Ignore")
      (`PrimitiveComponent.SetCollisionResponseToChannel` (`self.Mesh`) "ECC_Pawn" "ECR_Ignore")
      (`PrimitiveComponent.SetCollisionResponseToChannel` (`self.CapsuleComponent`) "ECC_WorldDynamic" "ECR_Ignore")
      (`PrimitiveComponent.SetCollisionResponseToChannel` (`self.CapsuleComponent`) "ECC_WorldStatic" "ECR_Ignore")
      (`PrimitiveComponent.SetCollisionResponseToChannel` (`self.CapsuleComponent`) "ECC_Camera" "ECR_Ignore")
      (`PrimitiveComponent.SetCollisionResponseToChannel` (`self.Mesh`) "ECC_Camera" "ECR_Ignore")
      (`PrimitiveComponent.SetCollisionEnabled` (`self.Mesh`) "QueryAndPhysics")
      (`NiagaraFunctionLibrary.SpawnSystemAtLocation` "/Game/Niagara/NS_HitEffect.NS_HitEffect" (`self.K2_GetActorLocation`))
      (`GameplayStatics.PlaySoundAtLocation` "/Game/Sounds/Placeholder/547041__cogfirestudios__hit-swing-sword-small-3.547041__cogfirestudios__hit-swing-sword-small-3" (`self.K2_GetActorLocation`) (struct) (`KismetMathLibrary.RandomFloatInRange` 1.0 1.2) (`KismetMathLibrary.RandomFloatInRange` 0.95 1.1) 0.0 null null null null)
      (`/Game/Player/Blueprints/BP_ThirdPersonCharacter.OnObjectiveIDCalled` (`self.PlayerRef`) (`self.ObjectiveID`) 1 true)
      (`PrimitiveComponent.AddImpulse` (`self.Mesh`) (+ (* (`self.GetActorForwardVector` (`self.PlayerRef`)) 3000.0) (0.0 0.0 50.0)) "None" false))))

(fn `PlayHitEffects`)

(fn `RemoveHelmet`)

(fn `SetMovementSpeed`
  (params (Speed :type "/Game/NPCs/Enemies/Data/E_EnemyMovementState Enum" :default "NewEnumerator0"))
  (returns (SpeedValue :type "Float (double-precision)"))
  (return 0.0))

(fn `UserConstructionScript`)