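; Zombie enemy character with a montage-driven melee attack, patrol route getter and idle, walking or running speed selection.
; Attack focuses on the player, plays the montage and signals completion when it finishes.
; A hit detector on the weapon socket damages the player reference on overlap during the montage's notify window, with a DoOnce limiting it to one hit until the window closes.
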(event `self.ReceiveBeginPlay`
  (`parent.ReceiveBeginPlay`)
  (set `self.ObjectiveID` "Zombie"))

(event `/Game/NPCs/Enemies/AI/Interfaces/BPI_EnemyAI.Attack_`
  (`AIController.K2_SetFocus` (`AIBlueprintHelperLibrary.GetAIController` self) (`GameplayStatics.GetPlayerCharacter` 0))
  (`|PlayMontage` (`self.Mesh`) "/Game/Lace/Chars/Zombies/ZombiemanTShirt/Anims/Zombie_Attack_Power_Montage.Zombie_Attack_Power_Montage" 2.0
    (:`OnCompleted`
      (`self.AttackComplete`))
    (:`OnNotifyBegin`
      (set `self.CanApplyDamage` true))
    (:`OnNotifyEnd`
      (set `self.CanApplyDamage` false)
      (goto _label :!via `Reset`))))

(event `self.HitDetector_.OnComponentBeginOverlap`
  (params (OverlappedComponent :type "PrimitiveComponent Object Reference") (OtherActor :type "Actor Object Reference") (OtherComp :type "PrimitiveComponent Object Reference") (OtherBodyIndex :type Integer) (bFromSweep :type Boolean) (SweepResult :type "HitResult Structure (by ref)"))
  ;[0 0 0] Apply damage. Checks if anything was in the HitDetector within the zombie's ApplyDamage window (dictated by the montage). When the damage window is closed, allow the zombie to deal damage again
  ;;[0.05 0.05 0.05] True if zombie isn't dead and its montage hit its notify
  (if (and (not (`self.isDead`)) (`self.CanApplyDamage`))
    (`/Engine/EditorBlueprintResources/StandardMacros.DoOnce` false :!label _label
      (:`Completed`
        (`GameplayStatics.ApplyDamage` (`self.PlayerStateRef`) (`self.Base Damage`) (`AIBlueprintHelperLibrary.GetAIController` self) self)))))

(fn `GetPatrolRoute`
  (returns (PatrolRoute :type "/Game/Blueprints/BP_PatrolRoute Object Reference") (`UsePatrolRoute?` :type Boolean))
  (return (`self.PatrolRoute`) (`self.UsePatrolRoute?`)))

(fn `SetMovementSpeed`
  (params (Speed :type "/Game/NPCs/Enemies/Data/E_EnemyMovementState Enum" :default "NewEnumerator0"))
  (returns (SpeedValue :type "Float (double-precision)"))
  (set `CharacterMovementComponent.MaxWalkSpeed` (select `/Game/NPCs/Enemies/Data/E_EnemyMovementState` Speed :`NewEnumerator1` (`self.MaxWalkingSpeed`) :`NewEnumerator2` (`self.MaxRunningSpeed`) :!type "Float (single-precision)") (`self.CharacterMovement`))
  (return 0.0))

(fn `UserConstructionScript`
  (`parent.UserConstructionScript`)
  (`SceneComponent.K2_AttachToComponent` (`self.HitDetector_`) (`self.Mesh`) "WeaponSocket" "KeepRelative" "KeepRelative" "KeepRelative" true))