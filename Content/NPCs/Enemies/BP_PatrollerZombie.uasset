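; Patrolling zombie enemy that AI-moves along the points of an assigned PatrolRoute spline.
; On BeginPlay it starts at the first point; each successful move steps the index by Direction, then delays briefly before the next move.
; Overrunning either end clamps the index and flips Direction but issues no further move, and destinations use spline-local coordinates.
; GetPatrolRoute returns the route with UsePatrolRoute false; parent BeginPlay is never called.
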(event `self.ReceiveBeginPlay`
  (bind _patrolroute (`self.PatrolRoute`))
  (`/Engine/EditorBlueprintResources/StandardMacros.IsValid` _patrolroute
    (:`Is Valid`
      (bind _output_get (set `self.NumberOfPoints` (`SplineComponent.GetNumberOfSplinePoints` (`/Game/Blueprints/BP_PatrolRoute.PatrolRoute` _patrolroute))))
      (if (> _output_get 0)
        (set `self.PatrolIndex` 0)
        (set `self.Direction` 1)
        (`self.MoveToNextSplinePoint`)
        (else
          (`KismetSystemLibrary.PrintString` "No spline points defined"))))))

(event `MoveToNextSplinePoint`
  (`|AIMoveTo` self (`SplineComponent.GetLocationAtSplinePoint` (`/Game/Blueprints/BP_PatrolRoute.PatrolRoute` (`self.PatrolRoute`)) (`self.PatrolIndex`) "Local") null 10.0
    (:`OnSuccess`
      (`self.IncrementPatrolRoute`))
    (:`OnFail`
      (`KismetSystemLibrary.PrintString` "AI Failed to move" true true (struct :`R` 1.0 :`B` 0.942791 :`A` 1.0)))))

(event `IncrementPatrolRoute`
  (set `self.PatrolIndex` (+ (`self.PatrolIndex`) (`self.Direction`)))
  (if (>= (`self.PatrolIndex`) (`self.NumberOfPoints`))
    (set `self.PatrolIndex` (- (`self.NumberOfPoints`) 1))
    (set `self.Direction` -1)
    (elif (< (`self.PatrolIndex`) 0)
      (set `self.PatrolIndex` 0)
      (set `self.Direction` 1)
      (else
        (`KismetSystemLibrary.Delay` 1.0)
        (`self.MoveToNextSplinePoint`)))))

(fn `GetPatrolRoute`
  (returns (PatrolRoute :type "/Game/Blueprints/BP_PatrolRoute Object Reference") (`UsePatrolRoute?` :type Boolean))
  (return (`self.PatrolRoute`) false))

(fn `UserConstructionScript`
  (`parent.UserConstructionScript`))