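; Player state Blueprint that tracks the player's health, inventory, equipped item and weapon ammo, and drives the HUD.
; On begin play it caches HUD and character references after a short delay, then seeds the inventory from DT_Items.
; Damage lowers attribute-set health, and death ragdolls the character while a timeline fades global time dilation toward zero.
; Helper functions handle hotbar highlighting, ammo decrement and magazine reloads from inventory.
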(event `self.ReceiveBeginPlay`
  (bind _hud_ref (`self.HUD_Ref`))
  (add `self.OnTakeAnyDamage` (delegate `OnTakeAnyDamage_Event`))
  (`KismetSystemLibrary.Delay` 0.2)
  (`self.SetReferences`)
  (`self.AddStartingItems`)
  (`/Game/UI/Common/Widgets/HUD/WB_Common_MainHUD.SetHealthBar` _hud_ref)
  (`/Game/UI/Common/Widgets/HUD/WB_Common_MainHUD.SetStaminaBar` _hud_ref))

(event `OnTakeAnyDamage_Event` :!signature `self.OnTakeAnyDamage`
  (params (DamagedActor :type "Actor Object Reference") (Damage :type "Float (single-precision)") (DamageType :type "DamageType Object Reference") (InstigatedBy :type "Controller Object Reference") (DamageCauser :type "Actor Object Reference"))
  (bind _hud_ref (`self.HUD_Ref`))
  (`/Game/Blueprints/Components/AC_BaseAttributeSet.ReduceHealth` (`self.AC_BaseAttributeSet`) Damage)
  (`/Game/UI/Common/Widgets/HUD/WB_Common_MainHUD.SetHealthBar` (`self.HUD_Ref`))
  (`UserWidget.PlayAnimation` _hud_ref (`/Game/UI/Common/Widgets/HUD/WB_Common_MainHUD.TookDamage` _hud_ref) 0.0 1 "Forward" 1.0 false)
  (if (<= (`/Game/Blueprints/Components/AC_BaseAttributeSet.GetHealth` (`self.AC_BaseAttributeSet`)) 0.0)
    (`self.OnDeath`)))

(event `OnDeath`
  (bind _as_bp_third_person_character (`self.As BP Third Person Character`))
  (bind _mesh (`Character.Mesh` _as_bp_third_person_character))
  (`/Engine/EditorBlueprintResources/StandardMacros.DoOnce` false
    (:`Completed`
      (`CharacterMovementComponent.SetMovementMode` (`Character.CharacterMovement` _as_bp_third_person_character) "MOVE_None" 0)
      (`PrimitiveComponent.SetCollisionProfileName` _mesh "Ragdoll" false)
      (`PrimitiveComponent.SetSimulatePhysics` _mesh true)
      (bind (_direction _alpha) (`Timeline|Timeline`)
        (:`Update`
          (`GameplayStatics.SetGlobalTimeDilation` (`KismetMathLibrary.Lerp` 1.0 0.0 _alpha)))))))

(event `SetHealthBar`
  (`/Game/UI/Common/Widgets/HUD/WB_Common_MainHUD.SetHealthBar` (`self.HUD_Ref`)))

(fn `AddStartingItems`
  (bind _returnvalue (`|GetDataTableRow` "/Game/Blueprints/Inventory/Data/DT_Items.DT_Items" "3")
    (:`then`
      (bind _structout (setmembers `/Game/Blueprints/Inventory/Data/Struct_Item` :`StructRef` _returnvalue :`PickedUpLocation` "NewEnumerator2" :`AmmoInWeapon` 12))
      (`/Game/Blueprints/Inventory/AC_InventoryComponent.Add` (`self.BP_InventoryComponent`) (make `/Game/Blueprints/Inventory/Data/Struct_InventorySlotData` _structout 1) false null)
      (bind _returnvalue_2 (`|GetDataTableRow` "/Game/Blueprints/Inventory/Data/DT_Items.DT_Items" "12")
        (:`then`
          (bind _structout_2 (setmembers `/Game/Blueprints/Inventory/Data/Struct_Item` :`StructRef` _returnvalue_2 :`PickedUpLocation` "NewEnumerator2" :`AmmoInWeapon` 21))
          (`/Game/Blueprints/Inventory/AC_InventoryComponent.Add` (`self.BP_InventoryComponent`) (make `/Game/Blueprints/Inventory/Data/Struct_InventorySlotData` _structout_2 1) false null)
          (bind _returnvalue_3 (`|GetDataTableRow` "/Game/Blueprints/Inventory/Data/DT_Items.DT_Items" "1")
            (:`then`
              (bind _structout_3 (setmembers `/Game/Blueprints/Inventory/Data/Struct_Item` :`StructRef` _returnvalue_3 :`PickedUpLocation` "NewEnumerator2"))
              (`/Game/Blueprints/Inventory/AC_InventoryComponent.Add` (`self.BP_InventoryComponent`) (make `/Game/Blueprints/Inventory/Data/Struct_InventorySlotData` _structout_3 1) false null)
              (bind _returnvalue_4 (`|GetDataTableRow` "/Game/Blueprints/Inventory/Data/DT_Items.DT_Items" "14")
                (:`then`
                  (bind _structout_4 (setmembers `/Game/Blueprints/Inventory/Data/Struct_Item` :`StructRef` _returnvalue_4 :`PickedUpLocation` "NewEnumerator2"))
                  (`/Game/Blueprints/Inventory/AC_InventoryComponent.Add` (`self.BP_InventoryComponent`) (make `/Game/Blueprints/Inventory/Data/Struct_InventorySlotData` _structout_4 500) false null)
                  (bind _returnvalue_5 (`|GetDataTableRow` "/Game/Blueprints/Inventory/Data/DT_Items.DT_Items" "13")
                    (:`then`
                      (bind _structout_5 (setmembers `/Game/Blueprints/Inventory/Data/Struct_Item` :`StructRef` _returnvalue_5 :`PickedUpLocation` "NewEnumerator2"))
                      (`/Game/Blueprints/Inventory/AC_InventoryComponent.Add` (`self.BP_InventoryComponent`) (make `/Game/Blueprints/Inventory/Data/Struct_InventorySlotData` _structout_5 50) false null)
                      (bind _returnvalue_6 (`|GetDataTableRow` "/Game/Blueprints/Inventory/Data/DT_Items.DT_Items" "2")
                        (:`then`
                          (bind _structout_6 (setmembers `/Game/Blueprints/Inventory/Data/Struct_Item` :`StructRef` _returnvalue_6 :`PickedUpLocation` "NewEnumerator2"))
                          (`/Game/Blueprints/Inventory/AC_InventoryComponent.Add` (`self.BP_InventoryComponent`) (make `/Game/Blueprints/Inventory/Data/Struct_InventorySlotData` _structout_6 50) false null)
                          (bind _returnvalue_7 (`|GetDataTableRow` "/Game/Blueprints/Inventory/Data/DT_Items.DT_Items" "15")
                            (:`then`
                              (bind _structout_7 (setmembers `/Game/Blueprints/Inventory/Data/Struct_Item` :`StructRef` _returnvalue_7 :`PickedUpLocation` "NewEnumerator2"))
                              (`/Game/Blueprints/Inventory/AC_InventoryComponent.Add` (`self.BP_InventoryComponent`) (make `/Game/Blueprints/Inventory/Data/Struct_InventorySlotData` _structout_7 50) false null)
                              (bind _returnvalue_8 (`|GetDataTableRow` "/Game/Blueprints/Inventory/Data/DT_Items.DT_Items" "16")
                                (:`then`
                                  (bind _structout_8 (setmembers `/Game/Blueprints/Inventory/Data/Struct_Item` :`StructRef` _returnvalue_8 :`PickedUpLocation` "NewEnumerator2"))
                                  (`/Game/Blueprints/Inventory/AC_InventoryComponent.Add` (`self.BP_InventoryComponent`) (make `/Game/Blueprints/Inventory/Data/Struct_InventorySlotData` _structout_8 50) false null))))))))))))))))))

(fn `BackendReload`
  (locals (FoundAmmoFromPlayerInventory :type "/Game/Blueprints/Inventory/Data/Struct_InventorySlotData Structure"))
  (bind _foundammofromplayerinventory_item (break `/Game/Blueprints/Inventory/Data/Struct_InventorySlotData` (`local.FoundAmmoFromPlayerInventory`)))
  (bind (_weaponmesh _damagemin _damagemax _ammocapacity) (break `/Game/Blueprints/Weapons/Data/Struct_WeaponData` (`.WeaponData_48_FC9EB35745BA4E0DC85F27AD67948517` (break `/Game/Blueprints/Inventory/Data/Struct_Item` (`self.EquippedItemObject`)))))
  (bind (_wasitemfound _fromhotbar _founditem) (`/Game/Blueprints/Inventory/AC_InventoryComponent.FindItem` (`self.BP_InventoryComponent`) (make `/Game/Blueprints/Inventory/Data/Struct_Item` (`.AmmoItemID_56_D1C4811C4489F62C67C489B68BE1897D` (break `/Game/Blueprints/Weapons/Data/Struct_WeaponData` (`.WeaponData_48_FC9EB35745BA4E0DC85F27AD67948517` (break `/Game/Blueprints/Inventory/Data/Struct_Item` (`self.EquippedItemObject`))))) "None" null null "" null "NewEnumerator0" false null null)))
  (if _wasitemfound
    (bind _output_get (set `local.FoundAmmoFromPlayerInventory` _founditem))
    (if (>= (`.Quantity_5_8D1E399245DFF28C8697A8BA5EC5307F` (break `/Game/Blueprints/Inventory/Data/Struct_InventorySlotData` _output_get)) (`.AmmoCapacity_30_9A9CBEBE4B48E93B6BCBB98A564E75CF` (break `/Game/Blueprints/Weapons/Data/Struct_WeaponData` (`.WeaponData_48_FC9EB35745BA4E0DC85F27AD67948517` (break `/Game/Blueprints/Inventory/Data/Struct_Item` (`self.EquippedItemObject`))))))
      (bind _structout (setmembers `/Game/Blueprints/Inventory/Data/Struct_Item` :`StructRef` (`self.EquippedItemObject`) :`AmmoInWeapon` _ammocapacity))
      (`/Game/Blueprints/Inventory/AC_InventoryComponent.Add` (`self.BP_InventoryComponent`) (make `/Game/Blueprints/Inventory/Data/Struct_InventorySlotData` _structout) false null)
      (`/Game/Blueprints/Inventory/AC_InventoryComponent.Remove` (`self.BP_InventoryComponent`) (make `/Game/Blueprints/Inventory/Data/Struct_InventorySlotData` _foundammofromplayerinventory_item _ammocapacity) false null)
      (else
        (`KismetSystemLibrary.PrintString` "Not enough ammo")
        (return)))
    (else
      (`KismetSystemLibrary.PrintString` "You don't have any ammo for that weapon")
      (return))))

(fn `DecrementAmmoInWeapon`
  (returns (AmmoRemaining :type Integer))
  (bind _result (`/Engine/EditorBlueprintResources/StandardMacros.DecrementInt` (`.AmmoInWeapon_65_8DF5FAF94899A8E2657C4893D822F6F7` (break `/Game/Blueprints/Inventory/Data/Struct_Item` (`self.EquippedItemObject`))))
    (:`  `
      (bind _structout (setmembers `/Game/Blueprints/Inventory/Data/Struct_Item` :`StructRef` (`self.EquippedItemObject`) :`AmmoInWeapon` _result))
      (`/Game/Blueprints/Inventory/AC_InventoryComponent.Add` (`self.BP_InventoryComponent`) (make `/Game/Blueprints/Inventory/Data/Struct_InventorySlotData` _structout) false null)
      (return _result))))

(fn `FindHotbarItem`
  (params (SlotIndex :type "Integer (by ref)"))
  (returns (Item :type "/Game/Blueprints/Inventory/Data/Struct_InventorySlotData Structure"))
  (return (`BlueprintMapLibrary.Map_Find` (`/Game/Blueprints/Inventory/AC_InventoryComponent.HotbarInventory` (`self.BP_InventoryComponent`)) SlotIndex)))

(fn `HighlightHotbarSlot`
  (params (SlotIndex :type Integer))
  (locals (FoundSlot :type "/Game/UI/Common/Inventory/Widgets/WB_InventorySlot Object Reference"))
  (bind _foundslot (`local.FoundSlot`))
  (bind _bp_inventorybutton (`/Game/UI/Common/Inventory/Widgets/WB_InventorySlot.BP_InventoryButton` _foundslot))
  (for (_array_element _array_index) (`/Game/UI/Common/Inventory/Widgets/WB_Hotbar.SlotArray` (`/Game/UI/Common/Widgets/HUD/WB_Common_MainInteractableHUD.WB_Hotbar` (`self.InteractableHUDRef`)))
    (if (== _array_index (`local.SlotIndex`))
      (set `local.FoundSlot` _array_element)
      (break)))
  (`UserWidget.PlayAnimation` _foundslot (`/Game/UI/Common/Inventory/Widgets/WB_InventorySlot.Select` _foundslot) 0.0 1 "Forward" 1.0 false)
  (set `/Game/UI/Common/Inventory/Buttons/BP_InventoryButton.isActive` true _bp_inventorybutton)
  (`CommonButtonBase.SetStyle` _bp_inventorybutton (`self.ActiveButtonStyle`)))

(fn `IsCurrentMagazineFull?`
  (returns (isFull :type Boolean))
  (locals (FoundAmmoFromPlayerInventory :type "/Game/Blueprints/Inventory/Data/Struct_InventorySlotData Structure"))
  (bind (_id _name _icon _staticmesh _description _actor _equip _isvalid _pickupsound _pickupeffect _pickeduplocation _buyselldata _isweapon _isconsumable _ammoinweapon _weapondata) (break `/Game/Blueprints/Inventory/Data/Struct_Item` (`self.EquippedItemObject`)))
  ;[0 0 0] True if weapon's magazine is full of ammo
  (if (>= _ammoinweapon (`.AmmoCapacity_30_9A9CBEBE4B48E93B6BCBB98A564E75CF` (break `/Game/Blueprints/Weapons/Data/Struct_WeaponData` _weapondata)))
    (return true)
    (else
      (return false))))

(fn `ReduceHealth`
  (params (Damage :type "Float (double-precision)")))

(fn `SetEquippedItem`
  (params (Item :type "/Game/Blueprints/Inventory/Data/Struct_Item Structure"))
  (set `self.EquippedItem` (`.Equip_43_37EA93F8450D8D45DA6BD2ADB1358281` (break `/Game/Blueprints/Inventory/Data/Struct_Item` Item)))
  (bind _output_get (set `self.EquippedItemObject` Item))
  (`KismetSystemLibrary.PrintString` (`KismetStringLibrary.Conv_NameToString` (`.Name_14_C95CFCF64759A9A970023A9D772B33CA` (break `/Game/Blueprints/Inventory/Data/Struct_Item` _output_get))))
  (return))

(fn `SetLastEquippedSlotInactive`
  (locals (FoundIndex :type Integer) (FoundSlot :type "/Game/UI/Common/Inventory/Widgets/WB_InventorySlot Object Reference"))
  (bind _foundslot (`local.FoundSlot`))
  (for (_array_element _array_index) (`/Game/UI/Common/Inventory/Widgets/WB_Hotbar.SlotArray` (`/Game/UI/Common/Widgets/HUD/WB_Common_MainInteractableHUD.WB_Hotbar` (`self.InteractableHUDRef`)))
    (if (== _array_index (`self.LastEquippedSlot`))
      (set `local.FoundSlot` _array_element)
      (break)))
  (`/Engine/EditorBlueprintResources/StandardMacros.IsValid` _foundslot
    (:`Is Valid`
      (`CommonButtonBase.SetStyle` (`/Game/UI/Common/Inventory/Widgets/WB_InventorySlot.BP_InventoryButton` _foundslot) (`self.InactiveButtonStyle`)))))

(fn `SetReferences`
  (bind _foundwidgets (`WidgetBlueprintLibrary.GetAllWidgetsOfClass` "/Game/UI/Common/Widgets/HUD/WB_Common_MainHUD.WB_Common_MainHUD_C" false))
  (set `self.HUD_Ref` (`|GetArrayItem` _foundwidgets))
  (bind _foundwidgets_2 (`WidgetBlueprintLibrary.GetAllWidgetsOfClass` "/Game/UI/Common/Widgets/HUD/WB_Common_MainInteractableHUD.WB_Common_MainInteractableHUD_C" false))
  (set `self.InteractableHUDRef` (`|GetArrayItem` _foundwidgets_2))
  (bind _asbp_third_person_character (cast `/Game/Player/Blueprints/BP_ThirdPersonCharacter` (`GameplayStatics.GetPlayerCharacter` 0)))
  (set `self.As BP Third Person Character` _asbp_third_person_character))

(fn `UNHighlightHotbarSlot`
  (params (SlotIndex :type Integer))
  (locals (FoundSlot :type "/Game/UI/Common/Inventory/Widgets/WB_InventorySlot Object Reference"))
  (bind _foundslot (`local.FoundSlot`))
  (bind _bp_inventorybutton (`/Game/UI/Common/Inventory/Widgets/WB_InventorySlot.BP_InventoryButton` _foundslot))
  (for (_array_element _array_index) (`/Game/UI/Common/Inventory/Widgets/WB_Hotbar.SlotArray` (`/Game/UI/Common/Widgets/HUD/WB_Common_MainInteractableHUD.WB_Hotbar` (`self.InteractableHUDRef`)))
    (if (== _array_index (`local.SlotIndex`))
      (set `local.FoundSlot` _array_element)
      (break)))
  (`CommonButtonBase.SetStyle` _bp_inventorybutton (`self.InactiveButtonStyle`))
  (set `/Game/UI/Common/Inventory/Buttons/BP_InventoryButton.isActive` false _bp_inventorybutton)
  (`UserWidget.PlayAnimation` _foundslot (`/Game/UI/Common/Inventory/Widgets/WB_InventorySlot.Deselect` _foundslot) 0.0 1 "Forward" 1.0 false))

(fn `UserConstructionScript`)