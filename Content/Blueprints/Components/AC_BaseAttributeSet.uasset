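; Actor component that stores an actor's health, stamina and money in a single BaseAttributes struct.
; BeginPlay fills current health and stamina to their maximums, and helper functions read and adjust values or check stamina state.
; Only AddHealth clamps, using the added amount as its minimum and MaxHealth as its maximum.
; AddMoney also fires the AddedMoney dispatcher with the owner.
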(event `self.ReceiveBeginPlay`
  (bind ((`MaxHealth_5_D888674D434D69F74FB08CA7C0F0673F` _maxhealth) (`MaxStamina_9_960D02DE4687EE568039E38FC5FDE5C2` _maxstamina)) (break `/Game/Blueprints/Components/Data/Struct_BaseAttributes` (`self.Attributes`)))
  (bind _structout (setmembers `/Game/Blueprints/Components/Data/Struct_BaseAttributes` :`StructRef` (`self.Attributes`) :`CurrentHealth` _maxhealth :`CurrentStamina` _maxstamina))
  (set `self.Attributes` _structout))

(fn `AddHealth`
  (params (Health :type "Float (double-precision)"))
  (bind _health (`local.Health`))
  (bind (_currenthealth _maxhealth) (break `/Game/Blueprints/Components/Data/Struct_BaseAttributes` (`self.Attributes`)))
  (bind _structout (setmembers `/Game/Blueprints/Components/Data/Struct_BaseAttributes` :`StructRef` (`self.Attributes`) :`CurrentHealth` (`KismetMathLibrary.FClamp` (+ _currenthealth _health) _health _maxhealth)))
  (set `self.Attributes` _structout))

(fn `AddMoney`
  (params (Money :type Integer))
  (bind _structout (setmembers `/Game/Blueprints/Components/Data/Struct_BaseAttributes` :`StructRef` (`self.Attributes`) :`Money` (+ (`.Money_12_B37CF06A4324ED17D9E2E281E8593509` (break `/Game/Blueprints/Components/Data/Struct_BaseAttributes` (`self.Attributes`))) (`local.Money`))))
  (set `self.Attributes` _structout)
  (`self.AddedMoney` (`self.GetOwner`)))

(fn `AddStamina`
  (params (Stamina :type "Float (double-precision)"))
  (bind _structout (setmembers `/Game/Blueprints/Components/Data/Struct_BaseAttributes` :`StructRef` (`self.Attributes`) :`CurrentStamina` (+ (`.CurrentStamina_7_22C78CD048EF1BE3F07F66A2F1BD625C` (break `/Game/Blueprints/Components/Data/Struct_BaseAttributes` (`self.Attributes`))) (`local.Stamina`))))
  (set `self.Attributes` _structout))

(fn `GetHealth`
  (returns (CurrentHealth :type "Float (double-precision)") (MaxHealth :type "Float (double-precision)"))
  (bind (_currenthealth _maxhealth) (break `/Game/Blueprints/Components/Data/Struct_BaseAttributes` (`self.Attributes`)))
  (return _currenthealth _maxhealth))

(fn `GetMoney`
  (returns (Money :type Integer))
  (return (`.Money_12_B37CF06A4324ED17D9E2E281E8593509` (break `/Game/Blueprints/Components/Data/Struct_BaseAttributes` (`self.Attributes`)))))

(fn `GetStamina`
  (returns (CurrentStamina :type "Float (double-precision)") (MaxStamina :type "Float (double-precision)"))
  (bind (_currenthealth _maxhealth _currentstamina _maxstamina) (break `/Game/Blueprints/Components/Data/Struct_BaseAttributes` (`self.Attributes`)))
  (return _currentstamina _maxstamina))

(fn `hasStamina`
  (returns (ReturnValue :type Boolean))
  (return (> (`self.GetStamina`) 0.0)))

(fn `isStaminaFull`
  (returns (isStaminaFull :type Boolean))
  (bind (_currenthealth _maxhealth _currentstamina _maxstamina) (break `/Game/Blueprints/Components/Data/Struct_BaseAttributes` (`self.Attributes`)))
  (return (>= _currentstamina _maxstamina)))

(fn `ReduceHealth`
  (params (Damage :type "Float (double-precision)"))
  (bind _structout (setmembers `/Game/Blueprints/Components/Data/Struct_BaseAttributes` :`StructRef` (`self.Attributes`) :`CurrentHealth` (- (`.CurrentHealth_4_08A009AF41BE28E802440C89655F69BB` (break `/Game/Blueprints/Components/Data/Struct_BaseAttributes` (`self.Attributes`))) (`local.Damage`))))
  (set `self.Attributes` _structout))

(fn `ReduceStamina`
  (params (Stamina :type "Float (double-precision)"))
  (bind _structout (setmembers `/Game/Blueprints/Components/Data/Struct_BaseAttributes` :`StructRef` (`self.Attributes`) :`CurrentStamina` (- (`.CurrentStamina_7_22C78CD048EF1BE3F07F66A2F1BD625C` (break `/Game/Blueprints/Components/Data/Struct_BaseAttributes` (`self.Attributes`))) (`local.Stamina`))))
  (set `self.Attributes` _structout))

(fn `SubtractMoney`
  (params (Money :type Integer))
  (bind _structout (setmembers `/Game/Blueprints/Components/Data/Struct_BaseAttributes` :`StructRef` (`self.Attributes`) :`Money` (- (`.Money_12_B37CF06A4324ED17D9E2E281E8593509` (break `/Game/Blueprints/Components/Data/Struct_BaseAttributes` (`self.Attributes`))) (`local.Money`))))
  (set `self.Attributes` _structout))