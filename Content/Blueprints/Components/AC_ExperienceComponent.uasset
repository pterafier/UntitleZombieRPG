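; Actor component that tracks experience and reputation progression in a shared attributes struct.
; XP level-ups carry overflow, raise the next threshold and grant attribute points.
; Reputation levels move both ways, deriving new thresholds from the XP requirement rather than their own, and broadcast changes through dispatchers.
; On BeginPlay and reputation level-up, it adds stores and outposts from the current difficulty tier's DT_QuestDifficulties row to the accessible lists.
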(event `self.ReceiveBeginPlay`
  (`self.UpdateAccessibilityArrays`)
  (add `self.OnReputationLevelUp` (delegate `OnReputationLevelUp_Event`)))

(event `OnReputationLevelUp_Event`
  (`self.UpdateAccessibilityArrays`))

(event `self.ReceiveTick`
  (params (DeltaSeconds :type "Float (single-precision)")))

(fn `AddReputation`
  (params (Reputation :type Integer))
  (if (not (< Reputation 0))
    (bind _structout (setmembers `/Game/Blueprints/Components/Data/Struct_ExperienceAttributes` :`StructRef` (`self.XPAttributes`) :`Reputation` (+ (`.Reputation_16_4FBCF69A498CB64D36765DAE0633EBA4` (break `/Game/Blueprints/Components/Data/Struct_ExperienceAttributes` (`self.XPAttributes`))) (`local.Reputation`))))
    (bind _output_get (set `self.XPAttributes` _structout))
    (bind ((`Reputation_16_4FBCF69A498CB64D36765DAE0633EBA4` _reputation) (`ReputationRequiredForNextLevel_17_60B2A793495FCF67E4C87CBE85355C83` _reputationrequiredfornextlevel)) (break `/Game/Blueprints/Components/Data/Struct_ExperienceAttributes` _output_get))
    (if (>= _reputation _reputationrequiredfornextlevel)
      (`self.ReputationLevelUp`))
    (else
      (`self.RemoveReputation` (`local.Reputation`)))))

(fn `AddXP`
  (params (Experience :type Integer))
  (bind _structout (setmembers `/Game/Blueprints/Components/Data/Struct_ExperienceAttributes` :`StructRef` (`self.XPAttributes`) :`Experience` (+ (`.Experience_3_CB793ADE4B8F7771479EF3A07DEFF14F` (break `/Game/Blueprints/Components/Data/Struct_ExperienceAttributes` (`self.XPAttributes`))) (`local.Experience`))))
  (bind _output_get (set `self.XPAttributes` _structout))
  (bind (_experience _expriencerequiredfornextlevel) (break `/Game/Blueprints/Components/Data/Struct_ExperienceAttributes` _output_get))
  (if (>= _experience _expriencerequiredfornextlevel)
    (`self.XPLevelUp`)))

(fn `GetAvailableAttributePoints`
  (returns (AvailableAttributePoints :type Integer))
  (return (`.AvailableAttributePoints_9_FFD242C74F13478DF2E8C6BD3EBAC4E6` (break `/Game/Blueprints/Components/Data/Struct_ExperienceAttributes` (`self.XPAttributes`)))))

(fn `GetCurrentLevel`
  (returns (Level :type Integer))
  (return (`.Level_7_780EC46B4714CB61C099998BE5804A02` (break `/Game/Blueprints/Components/Data/Struct_ExperienceAttributes` (`self.XPAttributes`)))))

(fn `GetReputation`
  (returns (Reputation :type Integer))
  (return (`.Reputation_16_4FBCF69A498CB64D36765DAE0633EBA4` (break `/Game/Blueprints/Components/Data/Struct_ExperienceAttributes` (`self.XPAttributes`)))))

(fn `GetReputationLevel`
  (returns (ReputationLevel :type Integer))
  (return (`.ReputationLevel_19_04B12CDB461729F2D1AA808E651E991D` (break `/Game/Blueprints/Components/Data/Struct_ExperienceAttributes` (`self.XPAttributes`)))))

(fn `GetXP`
  (returns (Experience :type Integer))
  (return (`.Experience_3_CB793ADE4B8F7771479EF3A07DEFF14F` (break `/Game/Blueprints/Components/Data/Struct_ExperienceAttributes` (`self.XPAttributes`)))))

(fn `RemoveReputation`
  (params (Reputation :type Integer))
  (bind _structout (setmembers `/Game/Blueprints/Components/Data/Struct_ExperienceAttributes` :`StructRef` (`self.XPAttributes`) :`Reputation` (- (`local.Reputation`) (`.Reputation_16_4FBCF69A498CB64D36765DAE0633EBA4` (break `/Game/Blueprints/Components/Data/Struct_ExperienceAttributes` (`self.XPAttributes`))))))
  (bind _output_get (set `self.XPAttributes` _structout))
  (bind ((`Reputation_16_4FBCF69A498CB64D36765DAE0633EBA4` _reputation)) (break `/Game/Blueprints/Components/Data/Struct_ExperienceAttributes` _output_get))
  (if (<= _reputation 0)
    (`self.ReputationLevelDown` (* _reputation -1))))

(fn `ReputationLevelDown`
  (params (RemainderXP :type Integer))
  (locals (RemainderExperience :type Integer))
  (set `local.RemainderExperience` RemainderXP)
  (bind _result (`/Engine/EditorBlueprintResources/StandardMacros.DecrementInt` (`.ReputationLevel_19_04B12CDB461729F2D1AA808E651E991D` (break `/Game/Blueprints/Components/Data/Struct_ExperienceAttributes` (`self.XPAttributes`))))
    (:`  `
      (bind _structout (setmembers `/Game/Blueprints/Components/Data/Struct_ExperienceAttributes` :`StructRef` (`self.XPAttributes`) :`Reputation` (`local.RemainderExperience`) :`ReputationRequiredForNextLevel` (`KismetMathLibrary.FTrunc` (/ (`.ExprienceRequiredForNextLevel_5_3A620C254A9BE06293D632B2ED157E0D` (break `/Game/Blueprints/Components/Data/Struct_ExperienceAttributes` (`self.XPAttributes`))) (`self.ReputationRequiredForNextLevelMultiplier`))) :`ReputationLevel` _result))
      (set `self.XPAttributes` _structout)
      (`self.OnReputationLevelDown`))))

(fn `ReputationLevelUp`
  (locals (RemainderExperience :type Integer))
  (bind (_experience _expriencerequiredfornextlevel _level _availableattributepoints _spentattributepoints _reputation _reputationrequiredfornextlevel) (break `/Game/Blueprints/Components/Data/Struct_ExperienceAttributes` (`self.XPAttributes`)))
  (bind _returnvalue (- _reputation _reputationrequiredfornextlevel))
  (if (> _returnvalue 0)
    (set `local.RemainderExperience` _returnvalue)
    (else
      (set `local.RemainderExperience` 0)))
  (bind _result (`/Engine/EditorBlueprintResources/StandardMacros.IncrementInt` (`.ReputationLevel_19_04B12CDB461729F2D1AA808E651E991D` (break `/Game/Blueprints/Components/Data/Struct_ExperienceAttributes` (`self.XPAttributes`))))
    (:`  `
      (bind _structout (setmembers `/Game/Blueprints/Components/Data/Struct_ExperienceAttributes` :`StructRef` (`self.XPAttributes`) :`AvailableAttributePoints` 0 :`Reputation` (`local.RemainderExperience`) :`ReputationRequiredForNextLevel` (`KismetMathLibrary.FTrunc` (* (`.ExprienceRequiredForNextLevel_5_3A620C254A9BE06293D632B2ED157E0D` (break `/Game/Blueprints/Components/Data/Struct_ExperienceAttributes` (`self.XPAttributes`))) (`self.ReputationRequiredForNextLevelMultiplier`))) :`ReputationLevel` _result))
      (set `self.XPAttributes` _structout)
      (`self.OnReputationLevelUp`))))

(fn `UpdateAccessibilityArrays`
  (bind _returnvalue (`|GetDataTableRow` "/Game/Blueprints/Quests/Data/DT_QuestDifficulties.DT_QuestDifficulties" (`KismetStringLibrary.Conv_StringToName` (`KismetStringLibrary.Conv_IntToString` (`self.CurrentDifficultyTier`))))
    (:`then`
      (bind (_minbasemoney _maxbasemoney _minbasexp _maxbasexp _minbasereputationgain _maxbasereputationgain _minbasereputationloss _maxbasereputationloss _minnumberofitems _maxnumberofitems _maxdifficultythreshold _availablestoreids _availableoutpostids) (break `/Game/Blueprints/Quests/Data/Struct_QuestTierData` _returnvalue))
      (for _array_element _availablestoreids
        (`KismetArrayLibrary.Array_AddUnique` (`self.CurrentlyAccessibleStores`) _array_element))
      (for _array_element_2 _availableoutpostids
        (`KismetArrayLibrary.Array_AddUnique` (`self.CurrentlyAccessibleOutposts`) _array_element_2)))))

(fn `XPLevelUp`
  (locals (RemainderExperience :type Integer))
  (bind (_experience _expriencerequiredfornextlevel _level _availableattributepoints) (break `/Game/Blueprints/Components/Data/Struct_ExperienceAttributes` (`self.XPAttributes`)))
  (bind (_experience_2 _expriencerequiredfornextlevel_2) (break `/Game/Blueprints/Components/Data/Struct_ExperienceAttributes` (`self.XPAttributes`)))
  (bind _returnvalue (- _experience_2 _expriencerequiredfornextlevel_2))
  (if (> _returnvalue 0)
    (set `local.RemainderExperience` _returnvalue)
    (else
      (set `local.RemainderExperience` 0)))
  (bind _result (`/Engine/EditorBlueprintResources/StandardMacros.IncrementInt` _level)
    (:`  `
      (bind _result_2 (`/Engine/EditorBlueprintResources/StandardMacros.IncrementInt` _availableattributepoints)
        (:`  `
          (bind _structout (setmembers `/Game/Blueprints/Components/Data/Struct_ExperienceAttributes` :`StructRef` (`self.XPAttributes`) :`Experience` (`local.RemainderExperience`) :`ExprienceRequiredForNextLevel` (`KismetMathLibrary.FTrunc` (* (`.ExprienceRequiredForNextLevel_5_3A620C254A9BE06293D632B2ED157E0D` (break `/Game/Blueprints/Components/Data/Struct_ExperienceAttributes` (`self.XPAttributes`))) 1.25)) :`Level` _result :`AvailableAttributePoints` _result_2))
          (set `self.XPAttributes` _structout)
          (`self.OnLevelUp`))))))