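; BP_SellChest is an interactable shop chest that opens a sell menu for the player.
; On interact it pushes WB_Common_SellMenu onto the base widget's menu stack and binds its own inventory component to the menu's other-inventory panel and slots.
; When looked at, it outlines the chest via custom depth stencil, using a per-frame timer to clear the highlight once the player looks away.
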(event `self.ReceiveBeginPlay`
  (set `/Game/Blueprints/Inventory/AC_InventoryComponent.OwnerOfInventory` self (`self.AC_InventoryComponent`))
  (`KismetSystemLibrary.Delay` 0.2)
  (`self.SetReferences`))

(event `/Game/Blueprints/Interfaces/BPI_Interact.LookAt`
  (`PrimitiveComponent.SetRenderCustomDepth` (`self.Chest`) true)
  (bind _returnvalue (`KismetSystemLibrary.K2_SetTimerDelegate` (delegate `UnHighlightMesh`) (`GameplayStatics.GetWorldDeltaSeconds`) true))
  (set `self.UnhighlightTimerHandle` _returnvalue)
  (`/Engine/EditorBlueprintResources/StandardMacros.DoOnce` false
    (:`Completed`
      (`PrimitiveComponent.SetCustomDepthStencilValue` (`self.Chest`) 250))))

(event `UnHighlightMesh`
  (if (not (== (`/Game/Player/Blueprints/BP_ThirdPersonCharacter.LookAtActor` (`self.Player Character Ref`)) self))
    (`PrimitiveComponent.SetRenderCustomDepth` (`self.Chest`) false)
    (`KismetSystemLibrary.K2_ClearAndInvalidateTimerHandle` (`self.UnhighlightTimerHandle`))))

(fn `Interact`
  (returns (ObjectiveID :type String))
  (bind _base_widget_ref (`self.Base Widget Ref`))
  (bind _ac_inventorycomponent (`self.AC_InventoryComponent`))
  (`/Game/UI/Common/Widgets/WB_Common_BaseWidget.PushWidgetToTargetStack` _base_widget_ref (`/Game/UI/Common/Widgets/WB_Common_BaseWidget.Menu_Stack` _base_widget_ref) "/Game/UI/Common/Widgets/Menus/WB_Common_SellMenu.WB_Common_SellMenu_C" true false)
  (bind _aswb_common_sell_menu (cast `/Game/UI/Common/Widgets/Menus/WB_Common_SellMenu` (`/Game/UI/Common/Widgets/WB_Common_BaseWidget.PushedWidget` (`self.Base Widget Ref`))))
  (bind _wb_otherinventory (`/Game/UI/Common/Widgets/Menus/WB_Common_SellMenu.WB_OtherInventory` _aswb_common_sell_menu))
  (`/Game/UI/Common/Inventory/Widgets/WB_OtherInventory.AssignDelegateOwnership` _wb_otherinventory _ac_inventorycomponent)
  (set `/Game/UI/Common/Inventory/Widgets/WB_OtherInventory.Owners Inventory` _ac_inventorycomponent _wb_otherinventory)
  (for _array_element (`/Game/UI/Common/Inventory/Widgets/WB_OtherInventory.OtherInventorySlotsArray` _wb_otherinventory)
    (set `/Game/UI/Common/Inventory/Widgets/WB_InventorySlot.OtherInventoryComponent` (`self.AC_InventoryComponent`) _array_element))
  (return (`self.ObjectiveID`)))

(fn `SetReferences`
  (set `self.Player State Ref` (`/Game/Blueprints/BFL_CommonFunctions.GetPlayerStateReference`))
  (set `self.Player Character Ref` (`/Game/Blueprints/BFL_CommonFunctions.GetPlayerCharacterReference`))
  (set `self.Base Widget Ref` (`/Game/Blueprints/BFL_CommonFunctions.GetBaseWidgetRef`)))

(fn `UserConstructionScript`)