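; Shop table that offers three random items for pickup, each with a quantity and price shown on text renders.
; On BeginPlay it draws from PossibleItems in a capped retry loop until three distinct items are found, then spawns a BP_SellerTablePickupItem at each spot.
; SetPrices rolls each price within its data table purchase range and passes it to the pickups.
; Pickup events refresh the quantity label, or hide both labels when stock runs out.
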(event `self.ReceiveBeginPlay`
  (set `self.ProductSlotsArray` (`|MakeArray` (`self.Spot1`) (`self.Spot2`) (`self.Spot3`)))
  (set `self.PriceTextRenderArray` (`|MakeArray` (`self.TextRender`) (`self.TextRender1`) (`self.TextRender2`)))
  (set `self.QtyTextRenderArray` (`|MakeArray` (`self.QuantityTextRender`) (`self.QtyTextRender`) (`self.QuantityTextRender1`)))
  (`self.GenerateShopItems`)
  (`self.SetPrices`))

(event `GenerateShopItems`
  (for _ (range 101)
    (bind _keys (`BlueprintMapLibrary.Map_Keys` (`self.PossibleItems`)))
    (bind (_outitem _outindex) (`KismetArrayLibrary.Array_Random` _keys))
    (if (not (`BlueprintMapLibrary.Map_Contains` (`self.DisplayedItemsMap`) _outitem))
      (bind _values (`BlueprintMapLibrary.Map_Values` (`self.PossibleItems`)))
      (`BlueprintMapLibrary.Map_Add` (`self.DisplayedItemsMap`) _outitem (`|GetArrayItem` _values _outindex))
      (if (== (`BlueprintMapLibrary.Map_Length` (`self.DisplayedItemsMap`)) 3)
        (break))))
  (for (_array_element _array_index) (`self.ProductSlotsArray`)
    (bind _keys_2 (`BlueprintMapLibrary.Map_Keys` (`self.DisplayedItemsMap`)))
    (bind _values_2 (`BlueprintMapLibrary.Map_Values` (`self.DisplayedItemsMap`)))
    (bind _returnvalue (`|SpawnActorFromClass` "/Game/Blueprints/Inventory/BP_SellerTablePickupItem.BP_SellerTablePickupItem_C" (`KismetMathLibrary.MakeTransform` (`SceneComponent.K2_GetComponentLocation` _array_element)) "Undefined" "MultiplyWithRoot" null 0 (`|GetArrayItem` _values_2 _array_index) (`|GetArrayItem` _keys_2 _array_index) null))
    (`KismetArrayLibrary.Array_Add` (`self.DisplayedPickupItems`) _returnvalue))
  (for (_array_element_2 _array_index_2) (`self.QtyTextRenderArray`)
    (bind _values_3 (`BlueprintMapLibrary.Map_Values` (`self.DisplayedItemsMap`)))
    (`TextRenderComponent.K2_SetText` _array_element_2 (`KismetTextLibrary.Conv_StringToText` (`KismetStringLibrary.Concat_StrStr` "x" (`KismetStringLibrary.Conv_IntToString` (`|GetArrayItem` _values_3 _array_index_2))))))
  (for _array_element_3 (`self.DisplayedPickupItems`)
    (add `/Game/Blueprints/Inventory/BP_PickupItem.ItemPickedUp` _array_element_3 (delegate `ItemPickedUp_Event_0`))))

(event `ItemPickedUp_Event_0`
  (params (ItemID :type Integer))
  (for (_array_element _array_index) (`self.DisplayedItems`)
    (if (== (`.ID_37_2860070F4E14361ABD215881AD40851C` (break `/Game/Blueprints/Inventory/Data/Struct_Item` _array_element)) ItemID)
      (bind _qty (`/Game/Blueprints/Inventory/BP_SellerTablePickupItem.Qty` (`|GetArrayItem` (`self.DisplayedPickupItems`) _array_index)))
      (if (> _qty 0)
        (`TextRenderComponent.K2_SetText` (`|GetArrayItem` (`self.QtyTextRenderArray`) _array_index) (`KismetTextLibrary.Conv_StringToText` (`KismetStringLibrary.Concat_StrStr` "x" (`KismetStringLibrary.Conv_IntToString` _qty))))
        (else
          (`SceneComponent.SetHiddenInGame` (`|GetArrayItem` (`self.PriceTextRenderArray`) _array_index) true false)
          (`SceneComponent.SetHiddenInGame` (`|GetArrayItem` (`self.QtyTextRenderArray`) _array_index) true false))))))

(fn `SetPrices`
  (bind _keys (`BlueprintMapLibrary.Map_Keys` (`self.DisplayedItemsMap`)))
  (for _array_element _keys
    (bind _founditem (`/Game/Blueprints/BFL_CommonFunctions.GetItemFromDataTable` _array_element))
    (bind (_purchaseprice_min _purchaseprice_max _purchaseprice_current _sellprice_current) (break `/Game/Blueprints/Inventory/Data/Struct_BuySellItemData` (`.BuySellData_72_5D0AD65E40761895FB05E0A48BCBFB14` (break `/Game/Blueprints/Inventory/Data/Struct_Item` _founditem))))
    (bind _structout (setmembers `/Game/Blueprints/Inventory/Data/Struct_Item` :`StructRef` _founditem :`BuySellData` (make `/Game/Blueprints/Inventory/Data/Struct_BuySellItemData` _purchaseprice_min _purchaseprice_max (`KismetMathLibrary.RandomIntegerInRange` _purchaseprice_min _purchaseprice_max) _sellprice_current)))
    (`KismetArrayLibrary.Array_AddUnique` (`self.DisplayedItems`) _structout))
  (for (_array_element_2 _array_index) (`self.DisplayedItems`)
    (`TextRenderComponent.K2_SetText` (`|GetArrayItem` (`self.PriceTextRenderArray`) _array_index) (`KismetTextLibrary.Conv_IntToText` (`.PurchasePrice_Current_6_D6ADD351477E9316955D609C942EEB94` (break `/Game/Blueprints/Inventory/Data/Struct_BuySellItemData` (`.BuySellData_72_5D0AD65E40761895FB05E0A48BCBFB14` (break `/Game/Blueprints/Inventory/Data/Struct_Item` _array_element_2)))))))
  (`self.UpdateShopItems`))

(fn `UpdateShopItems`
  (for (_array_element _array_index) (`self.DisplayedPickupItems`)
    (set `/Game/Blueprints/Inventory/BP_SellerTablePickupItem.Price` (`.PurchasePrice_Current_6_D6ADD351477E9316955D609C942EEB94` (break `/Game/Blueprints/Inventory/Data/Struct_BuySellItemData` (`.BuySellData_72_5D0AD65E40761895FB05E0A48BCBFB14` (break `/Game/Blueprints/Inventory/Data/Struct_Item` (`|GetArrayItem` (`self.DisplayedItems`) _array_index))))) _array_element)))

(fn `UserConstructionScript`)