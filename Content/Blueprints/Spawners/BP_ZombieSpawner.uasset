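; BP_ZombieSpawner is a spawner actor that releases a randomly sized group of BP_Zombie actors when play begins.
; BeginPlay rolls the count between configurable bounds and starts a short looping timer that spawns one zombie per tick until that count is reached, then clears itself.
; Each zombie spawns slightly above the spawner and receives its patrol route settings.
; SpawnSingleZombie provides an uncounted, on-demand spawn with the same setup.
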(event `self.ReceiveBeginPlay`
  (set `self.ZombiesToSpawn` (`KismetMathLibrary.RandomIntegerInRange` (`self.ZombiesToSpawnMIN`) (`self.ZombiesToSpawnMAX`)))
  (bind _returnvalue (`KismetSystemLibrary.K2_SetTimerDelegate` (delegate `AutoSpawnZombie`) 0.25 true))
  (set `self.TimerHandle` _returnvalue))

(event `AutoSpawnZombie`
  (if (< (`self.ZombiesSpawned`) (`self.ZombiesToSpawn`))
    (`|SpawnActorFromClass` "/Game/NPCs/Enemies/BP_Zombie.BP_Zombie_C" (`KismetMathLibrary.MakeTransform` (+ (`self.K2_GetActorLocation`) (0.0 0.0 50.0)) (`SceneComponent.K2_GetComponentRotation` (`self.DefaultSceneRoot`))) "AdjustIfPossibleButAlwaysSpawn" "MultiplyWithRoot" null (`self.PatrolRoute`) (`self.Use Patrol Route?`) null)
    (`/Engine/EditorBlueprintResources/StandardMacros.IncrementInt` (`self.ZombiesSpawned`))
    (else
      (`KismetSystemLibrary.K2_ClearAndInvalidateTimerHandle` (`self.TimerHandle`)))))

(event `SpawnSingleZombie`
  (`|SpawnActorFromClass` "/Game/NPCs/Enemies/BP_Zombie.BP_Zombie_C" (`KismetMathLibrary.MakeTransform` (+ (`self.K2_GetActorLocation`) (0.0 0.0 50.0)) (`SceneComponent.K2_GetComponentRotation` (`self.DefaultSceneRoot`))) "AdjustIfPossibleButAlwaysSpawn" "MultiplyWithRoot" null (`self.PatrolRoute`) (`self.Use Patrol Route?`) null))

(fn `UserConstructionScript`)