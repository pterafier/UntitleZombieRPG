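; Blueprint function library of shared helpers for player references, item lookup and reward granting.
; Getters return the index 0 character, state and controller cast to project classes, plus the first top-level base widget.
; GetItemFromDataTable treats ItemID as a 1-based row position in DT_Items, not a row name.
; AddRewards switches on reward type to feed the player state's experience, inventory or attribute components; an unconnected older reward loop remains.
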(fn `AddRewards`
  (params (Array :type "Array of /Game/Blueprints/Quests/Data/Struct_AllRewards Structure") (PlayerStateRef :type "/Game/Player/Blueprints/BP_PlayerState Object Reference"))
  (locals (Qty :type Integer) (ItemID :type Integer))
  (for _array_element Array
    (bind (_rewardtype _itemid _quantity) (break `/Game/Blueprints/Quests/Data/Struct_AllRewards` _array_element))
    (set `local.Qty` _quantity)
    (set `local.ItemID` _itemid)
    (switch `/Game/Blueprints/Quests/Data/E_RewardTypes` _rewardtype
      (:`NewEnumerator0`
        (`/Game/Blueprints/Components/AC_ExperienceComponent.AddXP` (`/Game/Player/Blueprints/BP_PlayerState.AC_ExperienceComponent` (`local.PlayerStateRef`)) (`local.Qty`)))
      (:`NewEnumerator1`
        (`/Game/Blueprints/Components/AC_ExperienceComponent.AddReputation` (`/Game/Player/Blueprints/BP_PlayerState.AC_ExperienceComponent` (`local.PlayerStateRef`)) (`local.Qty`)))
      (:`NewEnumerator2`
        (bind _founditem (`self.GetItemFromDataTable` (`local.ItemID`)))
        (`/Game/Blueprints/Inventory/AC_InventoryComponent.Add` (`/Game/Player/Blueprints/BP_PlayerState.BP_InventoryComponent` (`local.PlayerStateRef`)) (make `/Game/Blueprints/Inventory/Data/Struct_InventorySlotData` _founditem (`local.Qty`)) false null))
      (:`NewEnumerator3`
        (`/Game/Blueprints/Components/AC_BaseAttributeSet.AddMoney` (`/Game/Player/Blueprints/BP_PlayerState.AC_BaseAttributeSet` (`local.PlayerStateRef`)) (`local.Qty`))))))

(fn `GetBaseWidgetRef`
  (returns (BaseWidgetRef :type "/Game/UI/Common/Widgets/WB_Common_BaseWidget Object Reference"))
  (bind _foundwidgets (`WidgetBlueprintLibrary.GetAllWidgetsOfClass` null "/Game/UI/Common/Widgets/WB_Common_BaseWidget.WB_Common_BaseWidget_C"))
  (return (`|GetArrayItem` _foundwidgets)))

(fn `GetItemFromDataTable`
  (params (ItemID :type Integer))
  (returns (FoundItem :type "/Game/Blueprints/Inventory/Data/Struct_Item Structure") (ItemFound :type Boolean))
  (bind _outrownames (`DataTableFunctionLibrary.GetDataTableRowNames` "/Game/Blueprints/Inventory/Data/DT_Items.DT_Items"))
  (bind _returnvalue (`|GetDataTableRow` "/Game/Blueprints/Inventory/Data/DT_Items.DT_Items" (`|GetArrayItem` _outrownames (- ItemID 1)))
    (:`then`
      (return _returnvalue true))
    (:`RowNotFound`
      (return _returnvalue false))))

(fn `GetPlayerCharacterReference`
  (returns (PlayerCharacterRef :type "/Game/Player/Blueprints/BP_ThirdPersonCharacter Object Reference"))
  (bind _asbp_third_person_character (cast `/Game/Player/Blueprints/BP_ThirdPersonCharacter` (`GameplayStatics.GetPlayerCharacter` null)))
  (return _asbp_third_person_character))

(fn `GetPlayerControllerReference`
  (returns (PlayerControllerRef :type "/Game/Player/Blueprints/BP_PlayerController Object Reference"))
  (bind _asbp_player_controller (cast `/Game/Player/Blueprints/BP_PlayerController` (`GameplayStatics.GetPlayerController` null)))
  (return _asbp_player_controller))

(fn `GetPlayerStateReference`
  (returns (PlayerStateRef :type "/Game/Player/Blueprints/BP_PlayerState Object Reference"))
  (bind _asbp_player_state (cast `/Game/Player/Blueprints/BP_PlayerState` (`GameplayStatics.GetPlayerState` null)))
  (return _asbp_player_state))