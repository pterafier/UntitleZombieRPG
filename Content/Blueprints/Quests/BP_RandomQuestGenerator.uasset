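; Generates and runs a random pickup-and-delivery quest for an NPC customer, started automatically shortly after BeginPlay.
; Picks items, store and outpost from accessible data table rows, then derives estimated time and difficulty from distance and ratings.
; Objective ID callbacks track pickups and advance the stage, while a gated Tick timer feeds the tracker widget.
; EndQuest scales money, XP and reputation by speed and difficulty, removing reputation for very late deliveries, then resets.
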(event `self.ReceiveBeginPlay`
  (`self.SetReferences`)
  (`KismetSystemLibrary.Delay` 0.2)
  (`self.SetPossibleItemIDs`)
  (add `/Game/Blueprints/Components/AC_ExperienceComponent.OnReputationLevelUp` (`/Game/Player/Blueprints/BP_PlayerState.AC_ExperienceComponent` (`self.Player State Ref`)) (delegate `OnReputationLevelUp_Event`))
  (add `/Game/Player/Blueprints/BP_ThirdPersonCharacter.OnObjectiveIDCalled` (`self.Player Character Ref`) (delegate `OnObjectiveIDCalled_Event`))
  (`self.GenerateQuest`)
  (`KismetSystemLibrary.Delay` 1.0)
  (`self.StartQuest`)
  (`self.ManageUI`)
  (add `self.OnQuestProgressed` (delegate `OnQuestProgressed_Event`)))

(event `OnQuestProgressed_Event`
  (`self.ManageUI`))

(event `OnObjectiveIDCalled_Event`
  (params (ObjectiveID :type String) (Value :type Integer) (`NotifyObjectiveComplete?` :type Boolean))
  (if (and (>= (`self.QuestStage`) 1) (< (`self.QuestStage`) 2))
    (`self.Check for Quest Items` ObjectiveID)
    (if (`self.hasAllQuestItems`)
      (`/Engine/EditorBlueprintResources/StandardMacros.DoOnce` false
        (:`Completed`
          (`/Engine/EditorBlueprintResources/StandardMacros.IncrementInt` (`self.QuestStage`)
            (:`  `
              (`self.OnQuestProgressed`)
              (bind _storewaypointref (`self.StoreWaypointRef`)
                (:`then`
                  (`self.K2_DestroyActor` _storewaypointref))
                (:`else`)))))))))

(event `OnReputationLevelUp_Event`
  (`self.SetPossibleItemIDs`))

(event `self.ReceiveTick`
  (params (DeltaSeconds :type "Float (single-precision)"))
  (`/Engine/EditorBlueprintResources/StandardMacros.Gate` true :!label _label
    (:`Exit`
      (bind _output_get (set `self.TimeElapsed` (+ (`self.TimeElapsed`) (`GameplayStatics.GetWorldDeltaSeconds`))))
      (bind _dashertrackerref (`self.DasherTrackerRef`)
        (:`then`
          (bind _objectiveentryref (`/Game/UI/Common/Widgets/Popups/WB_Common_DasherQuestDetailsTracker.ObjectiveEntryRef` _dashertrackerref))
          (set `/Game/UI/Common/Widgets/Menus/Quests/WB_DasherQuest_ObjectiveEntry.TimerText` (`KismetTextLibrary.Conv_StringToText` (`KismetStringLibrary.Concat_StrStr` "Time elapsed: " (`KismetTextLibrary.Conv_TextToString` (`KismetTextLibrary.Conv_DoubleToText` _output_get "HalfToEven" false true 1 200 0 2)))) _objectiveentryref)
          (`/Game/UI/Common/Widgets/Menus/Quests/WB_DasherQuest_ObjectiveEntry.UpdateTimer` _objectiveentryref))
        (:`else`)))))

(event `StartQuestTimer`
  (goto _label :!via `Open`))

(event `StopQuestTimer`
  (goto _label :!via `Close`))

(fn `AddNormalRewardsToArray`
  (params (XPReward :type Integer) (MoneyReward :type Integer) (RepReward :type Integer))
  ;[0 0 0] Add XP reward to rewards array
  (bind _structout (setmembers `/Game/Blueprints/Quests/Data/Struct_AllRewards` :`StructRef` (`self.Reward`) :`RewardType` "NewEnumerator0" :`Quantity` XPReward))
  (`KismetArrayLibrary.Array_Add` (`self.Rewards`) _structout)
  ;[0 0 0] Add money to rewards array
  (bind _structout_2 (setmembers `/Game/Blueprints/Quests/Data/Struct_AllRewards` :`StructRef` (`self.Reward`) :`RewardType` "NewEnumerator3" :`Quantity` MoneyReward))
  (`KismetArrayLibrary.Array_Add` (`self.Rewards`) _structout_2)
  ;[0 0 0] Add rep reward to rewards array
  (setmembers `/Game/Blueprints/Quests/Data/Struct_AllRewards` :`StructRef` (`self.Reward`) :`RewardType` "NewEnumerator1" :`Quantity` RepReward)
  (`KismetArrayLibrary.Array_Add` (`self.Rewards`)))

(fn `CalculateAndAddRewards`
  (locals (DifficultyData_Local :type "/Game/Blueprints/Quests/Data/Struct_QuestTierData Structure") (MoneyReward :type Integer :default 0) (XPReward :type Integer :default 0) (ReputationReward :type Integer))
  (bind (_minbasemoney _maxbasemoney _minbasexp _maxbasexp _minbasereputationgain _maxbasereputationgain) (break `/Game/Blueprints/Quests/Data/Struct_QuestTierData` (`local.DifficultyData_Local`)))
  (bind (_minbasemoney_2 _maxbasemoney_2 _minbasexp_2 _maxbasexp_2) (break `/Game/Blueprints/Quests/Data/Struct_QuestTierData` (`local.DifficultyData_Local`)))
  (bind (_minbasemoney_3 _maxbasemoney_3 _minbasexp_3 _maxbasexp_3 _minbasereputationgain_2 _maxbasereputationgain_2 _minbasereputationloss _maxbasereputationloss) (break `/Game/Blueprints/Quests/Data/Struct_QuestTierData` (`local.DifficultyData_Local`)))
  (bind _returnvalue (`KismetMathLibrary.RandomIntegerInRange` _minbasereputationloss _maxbasereputationloss))
  ;[0 0 0] Get current difficulty tier data. This is the base information rewards are calculated by.
  (bind _returnvalue_2 (`|GetDataTableRow` "/Game/Blueprints/Quests/Data/DT_QuestDifficulties.DT_QuestDifficulties" (`KismetStringLibrary.Conv_StringToName` (`KismetStringLibrary.Conv_IntToString` (`/Game/Blueprints/Components/AC_ExperienceComponent.CurrentDifficultyTier` (`/Game/Player/Blueprints/BP_PlayerState.AC_ExperienceComponent` (`self.Player State Ref`))))))
    (:`then`
      (set `local.DifficultyData_Local` _returnvalue_2)
      ;[0 0 0] Compare the quests difficulty against the max difficulty threshold. If the quest is significantly harder than this tier's max difficulty threshold, set the multiplier to be higher with a maximum of 2
      (set `self.DifficultyMultiplier` (`KismetMathLibrary.FClamp` (`KismetMathLibrary.Conv_IntToDouble` (/ (`self.QuestDifficulty`) (`.MaxDifficultyThreshold_71_763D9E7440F7AD9E6A0B279A96D80606` (break `/Game/Blueprints/Quests/Data/Struct_QuestTierData` (`local.DifficultyData_Local`))))) 0.0 2.0))
      ;[0 0 0] Calculate how quickly the player completed the delivery. If they took significantly longer than the estimated delivery time, reputation will be reduced. The player will still earn money and XP no matter what, just with a much lower multiplier.
      (set `self.TimeMultiplier` (`KismetMathLibrary.FClamp` (/ (`self.EstimatedDeliveryTime`) (`self.TimeElapsed`)) 0.0 2.0))
      ;[0 0 0] Pick a random integer between the minimum and maximum rewards, then apply the multipliers to them (only for money and XP, reputation is evaluated below)
      (`|ExecutionSequence`
        (:`then_0`
          (bind _returnvalue_3 (`self.MultiplyRewards` _minbasemoney_2 _maxbasemoney_2))
          (set `local.MoneyReward` _returnvalue_3))
        (:`then_1`
          (bind _returnvalue_4 (`self.MultiplyRewards` _minbasexp_2 _maxbasexp_2))
          (set `local.XPReward` _returnvalue_4))
        (:`then_2`
          ;[0 0 0] The threshold where the player loses reputation. If they're significatnly slower than the estimated delivery time, reduce reputation.
          (if (< (`self.TimeMultiplier`) 0.5)
            (set `local.ReputationReward` (`KismetMathLibrary.FTrunc` (`KismetMathLibrary.FClamp` (* _returnvalue (- 2.0 (`self.TimeMultiplier`))) 0.0 (`KismetMathLibrary.Conv_IntToDouble` _returnvalue))))
            ;[0 0 0] Add XP reward to rewards array
            (bind _structout (setmembers `/Game/Blueprints/Quests/Data/Struct_AllRewards` :`StructRef` (`self.Reward`) :`RewardType` "NewEnumerator0" :`Quantity` (`local.XPReward`)))
            (`KismetArrayLibrary.Array_Add` (`self.Rewards`) _structout)
            ;[0 0 0] Add money to rewards array
            (bind _structout_2 (setmembers `/Game/Blueprints/Quests/Data/Struct_AllRewards` :`StructRef` (`self.Reward`) :`RewardType` "NewEnumerator3" :`Quantity` (`local.MoneyReward`)))
            (`KismetArrayLibrary.Array_Add` (`self.Rewards`) _structout_2)
            (`/Game/Blueprints/BFL_CommonFunctions.AddRewards` (`self.Rewards`) (`self.Player State Ref`))
            (`/Game/Blueprints/Components/AC_ExperienceComponent.RemoveReputation` (`/Game/Player/Blueprints/BP_PlayerState.AC_ExperienceComponent` (`self.Player State Ref`)) (`local.ReputationReward`))
            (`KismetSystemLibrary.PrintString` (`KismetStringLibrary.Concat_StrStr` "Money reward: " (`KismetStringLibrary.Conv_IntToString` (`local.MoneyReward`)) " \nXP Reward: " (`KismetStringLibrary.Conv_IntToString` (`local.XPReward`)) " \nReputation reward (Rep was removed): " (`KismetStringLibrary.Conv_IntToString` (`local.ReputationReward`))) true true (struct :`G` 0.66 :`B` 1.0 :`A` 1.0) 20.0)
            (else
              (bind _returnvalue_5 (`self.MultiplyRewards` _minbasereputationgain _maxbasereputationgain))
              (set `local.ReputationReward` _returnvalue_5)
              (`self.AddNormalRewardsToArray` (`local.XPReward`) (`local.MoneyReward`) (`local.ReputationReward`))
              (`/Game/Blueprints/BFL_CommonFunctions.AddRewards` (`self.Rewards`) (`self.Player State Ref`))
              (`KismetSystemLibrary.PrintString` (`KismetStringLibrary.Concat_StrStr` "Money reward: " (`KismetStringLibrary.Conv_IntToString` (`local.MoneyReward`)) " \nXP Reward: " (`KismetStringLibrary.Conv_IntToString` (`local.XPReward`)) " \nReputation reward: " (`KismetStringLibrary.Conv_IntToString` (`local.ReputationReward`))) true true (struct :`G` 0.66 :`B` 1.0 :`A` 1.0) 20.0))))))))

(fn `CalculateApproximateQuestDistance`
  (set `self.DistanceFromStoreToOutpost` (`self.GetDistanceTo` (`self.PreferredStore`) (`self.TargetOutpost`)))
  (set `self.DistanceFromPlayerToStore` (`self.GetDistanceTo` (`self.Player Character Ref`) (`self.PreferredStore`)))
  (set `self.TotalDistance_CM` (+ (`self.DistanceFromStoreToOutpost`) (`self.DistanceFromPlayerToStore`))))

(fn `CalculateQuestDifficulty`
  (locals (OutpostDifficulty_Local :type Integer) (StoreDifficulty_Local :type Integer))
  (bind _returnvalue (`|GetDataTableRow` "/Game/Blueprints/Quests/Data/DT_Outposts.DT_Outposts" (`KismetStringLibrary.Conv_StringToName` (`KismetStringLibrary.Conv_IntToString` (`self.OutpostID`))))
    (:`then`
      (set `local.OutpostDifficulty_Local` (`.OutpostDifficultyRating_11_6EF46F0846CE9CCBAC6BF2A86E2A6A47` (break `/Game/Blueprints/Quests/Data/Struct_Outpost` _returnvalue)))
      (bind _returnvalue_2 (`|GetDataTableRow` "/Game/Blueprints/Inventory/Data/DT_Stores.DT_Stores" (`KismetStringLibrary.Conv_StringToName` (`KismetStringLibrary.Conv_IntToString` (`self.PreferredStoreID`))))
        (:`then`
          (bind _output_get (set `local.StoreDifficulty_Local` (`.StoreDifficultyRating_40_92F5E15146CB908C558A89901DE40BE3` (break `/Game/Blueprints/Inventory/Data/Struct_Store` _returnvalue_2))))
          (set `self.QuestDifficulty` (+ (+ _output_get (`local.OutpostDifficulty_Local`) (`KismetMathLibrary.FTrunc` (/ (`self.EstimatedDeliveryTime`) 100.0))) (`self.NumberOfItems`))))))))

(fn `CalculateQuestDuration`
  (locals (OutpostTravelTime :type "Float (double-precision)"))
  (`self.CalculateApproximateQuestDistance`)
  ;[0 0 0] For each meter:
  (for _ (range 1 (+ (`KismetMathLibrary.FTrunc` (/ (`self.TotalDistance_CM`) 100.0)) 1))
    ;[0 0 0] Add x seconds to the estimated delivery time
    (set `self.EstimatedDeliveryTime` (+ (`self.EstimatedDeliveryTime`) 0.33)))
  (bind _returnvalue (`|GetDataTableRow` "/Game/Blueprints/Quests/Data/DT_Outposts.DT_Outposts" (`KismetStringLibrary.Conv_StringToName` (`KismetStringLibrary.Conv_IntToString` (`self.OutpostID`))))
    (:`then`
      (set `local.OutpostTravelTime` (`.TravelTime_14_100953664EB7BDA83113EC8D7A331A1D` (break `/Game/Blueprints/Quests/Data/Struct_Outpost` _returnvalue)))
      (bind _returnvalue_2 (`|GetDataTableRow` "/Game/Blueprints/Inventory/Data/DT_Stores.DT_Stores" (`KismetStringLibrary.Conv_StringToName` (`KismetStringLibrary.Conv_IntToString` (`self.PreferredStoreID`))))
        (:`then`
          (set `self.EstimatedDeliveryTime` (+ (`self.EstimatedDeliveryTime`) (`local.OutpostTravelTime`) (`.TravelTime_46_0363F465415C7C0D6D30FEB93CC509DA` (break `/Game/Blueprints/Inventory/Data/Struct_Store` _returnvalue_2)))))))))

(fn `Check for Quest Items`
  (params (ObjectiveID :type String))
  (for _array_element (`self.WantedItemIDs`)
    (if (`KismetStringLibrary.EqualEqual_StrStr` (`local.ObjectiveID`) (`KismetStringLibrary.Conv_IntToString` _array_element))
      (bind (_founditem _itemfound) (`/Game/Blueprints/BFL_CommonFunctions.GetItemFromDataTable` _array_element))
      (if _itemfound
        (`KismetArrayLibrary.Array_AddUnique` (`self.CollectedQuestItems`) _founditem)
        (else
          (`KismetSystemLibrary.PrintString` "Attempted to add item to CollectedQuestItems array, but could not find the item in the data table" true true (struct :`R` 1.0 :`B` 0.016654 :`A` 1.0) 30.0)))))
  (if (== (`KismetArrayLibrary.Array_Length` (`self.CollectedQuestItems`)) (`KismetArrayLibrary.Array_Length` (`self.WantedItems`)))
    (set `self.hasAllQuestItems` true)))

(fn `EndQuest`
  (`self.StopQuestTimer`)
  (`self.CalculateAndAddRewards`)
  (`self.RemoveQuestItemsFromPlayerInventory`)
  (`self.ResetVariables`)
  (`Widget.RemoveFromParent` (`self.DasherTrackerRef`)))

(fn `FormatItemsText`
  (returns (Result :type String))
  (for _array_element (`self.WantedItems`)
    (set `self.Result` (`KismetStringLibrary.Concat_StrStr` (`self.Result`) (`KismetStringLibrary.Conv_NameToString` (`.Name_14_C95CFCF64759A9A970023A9D772B33CA` (break `/Game/Blueprints/Inventory/Data/Struct_Item` _array_element))) ", ")))
  (return (`KismetStringLibrary.LeftChop` (`self.Result`) 2)))

(fn `GenerateCustomerDetails`
  (bind _outitem (`KismetArrayLibrary.Array_Random` (`/Game/Blueprints/Components/AC_ExperienceComponent.CurrentlyAccessibleOutposts` (`/Game/Player/Blueprints/BP_PlayerState.AC_ExperienceComponent` (`self.Player State Ref`)))))
  (bind _returnvalue (`|GetDataTableRow` "/Game/Blueprints/Quests/Data/DT_Outposts.DT_Outposts" (`KismetStringLibrary.Conv_StringToName` (`KismetStringLibrary.Conv_IntToString` _outitem)))
    (:`then`
      (bind _output (`|ConvertAsset` (`.OutpostActor_8_6C5136B94029BF52E46E089C2AD13E6E` (break `/Game/Blueprints/Quests/Data/Struct_Outpost` _returnvalue))))
      (bind _randomcustomer (`/Game/Blueprints/Shops/BP_Outpost.PickRandomCustomer` _output))
      (bind _asbp_npc_customer (cast `/Game/NPCs/BP_NPC_Customer` _randomcustomer))
      (set `self.TargetCustomer` _asbp_npc_customer)
      (set `self.TargetOutpost` _output)
      (set `self.OutpostID` _outitem)
      (set `/Game/NPCs/BP_NPC_Customer.isActiveCustomer` true _asbp_npc_customer))))

(fn `GenerateItemDetails`
  (bind _storeid (`self.GeneratePreferredStore`))
  (bind _returnvalue (`|GetDataTableRow` "/Game/Blueprints/Inventory/Data/DT_Stores.DT_Stores" (`KismetStringLibrary.Conv_StringToName` (`KismetStringLibrary.Conv_IntToString` _storeid)))
    (:`then`
      (set `self.NumberOfItems` (`self.GenerateNumberOfWantedItems`))
      (for _ (range 101)
        (bind (_id _name _storeactor _storeitems) (break `/Game/Blueprints/Inventory/Data/Struct_Store` _returnvalue))
        (bind _founditem (`/Game/Blueprints/BFL_CommonFunctions.GetItemFromDataTable` (`.ItemID_16_631064EE4BF40380D410ECBF1096056C` (break `/Game/Blueprints/Inventory/Data/Struct_StoreItem` (`KismetArrayLibrary.Array_Random` _storeitems)))))
        (`KismetArrayLibrary.Array_AddUnique` (`self.WantedItems`) _founditem)
        (`KismetArrayLibrary.Array_AddUnique` (`self.WantedItemIDs`) (`.ID_37_2860070F4E14361ABD215881AD40851C` (break `/Game/Blueprints/Inventory/Data/Struct_Item` _founditem)))
        (if (== (`KismetArrayLibrary.Array_Length` (`self.WantedItems`)) (`self.NumberOfItems`))
          (break)))
      (set `self.PreferredStore` (`|ConvertAsset` _storeactor))
      (set `self.PreferredStoreID` _storeid)
      (`KismetSystemLibrary.PrintString` (`KismetStringLibrary.Conv_IntToString` (`KismetArrayLibrary.Array_Length` (`self.WantedItems`))) true true (struct :`R` 1.0 :`G` 0.888586 :`A` 1.0) 12.0))))

(fn `GenerateNumberOfWantedItems`
  (returns (NumberOfItems :type Integer))
  (bind _returnvalue (`|GetDataTableRow` "/Game/Blueprints/Quests/Data/DT_QuestDifficulties.DT_QuestDifficulties" (`KismetStringLibrary.Conv_StringToName` (`KismetStringLibrary.Conv_IntToString` (`/Game/Blueprints/Components/AC_ExperienceComponent.CurrentDifficultyTier` (`/Game/Player/Blueprints/BP_PlayerState.AC_ExperienceComponent` (`self.Player State Ref`))))))
    (:`then`
      (bind (_minbasemoney _maxbasemoney _minbasexp _maxbasexp _minbasereputationgain _maxbasereputationgain _minbasereputationloss _maxbasereputationloss _minnumberofitems _maxnumberofitems) (break `/Game/Blueprints/Quests/Data/Struct_QuestTierData` _returnvalue))
      (return (`KismetMathLibrary.Clamp` (`KismetMathLibrary.RandomIntegerInRange` _minnumberofitems _maxnumberofitems) 1 _maxnumberofitems)))))

(fn `GeneratePreferredStore`
  (returns (StoreID :type Integer))
  (return (`KismetArrayLibrary.Array_Random` (`/Game/Blueprints/Components/AC_ExperienceComponent.CurrentlyAccessibleStores` (`/Game/Player/Blueprints/BP_PlayerState.AC_ExperienceComponent` (`self.Player State Ref`))))))

(fn `GenerateQuest`
  (`self.GenerateItemDetails`)
  (`self.GenerateCustomerDetails`)
  (`self.CalculateQuestDuration`)
  (`self.CalculateQuestDifficulty`)
  (`KismetSystemLibrary.PrintString` (`KismetStringLibrary.Concat_StrStr` "Quest difficulty rating: " (`KismetStringLibrary.Conv_IntToString` (`self.QuestDifficulty`)) " \nEstimated delivery time: " (`KismetStringLibrary.Conv_DoubleToString` (`self.EstimatedDeliveryTime`)) " \nApproximate distance: " (`KismetStringLibrary.Conv_DoubleToString` (`self.TotalDistance_CM`)) " \nNumber of items to pickup: " (`KismetStringLibrary.Conv_IntToString` (`self.NumberOfItems`)) " \nPreferred store: " (`KismetStringLibrary.Conv_IntToString` (`self.PreferredStoreID`))) true true (struct :`G` 0.66 :`B` 1.0 :`A` 1.0) 10.0))

(fn `ManageUI`
  (if (>= (`self.QuestStage`) 1)
    (bind _dashertrackerref (`self.DasherTrackerRef`)
      (:`then`
        (`/Game/UI/Common/Widgets/Popups/WB_Common_DasherQuestDetailsTracker.UpdateDasherTracker` _dashertrackerref))
      (:`else`
        (`/Engine/EditorBlueprintResources/StandardMacros.DoOnce` false
          (:`Completed`
            (bind _returnvalue (`|CreateWidget` "/Game/UI/Common/Widgets/Popups/WB_Common_DasherQuestDetailsTracker.WB_Common_DasherQuestDetailsTracker_C"))
            (bind _output_get (set `self.DasherTrackerRef` _returnvalue))
            (set `/Game/UI/Common/Widgets/Popups/WB_Common_DasherQuestDetailsTracker.RandomQuest_TitleText` "Order for NPC" _output_get)
            (bind _returnvalue_2 (`|GetDataTableRow` "/Game/Blueprints/Inventory/Data/DT_Stores.DT_Stores" (`KismetStringLibrary.Conv_StringToName` (`KismetStringLibrary.Conv_IntToString` (`self.PreferredStoreID`))))
              (:`then`
                (set `/Game/UI/Common/Widgets/Popups/WB_Common_DasherQuestDetailsTracker.RandomQuestStoreLocation Name` (`KismetTextLibrary.Conv_StringToText` (`KismetStringLibrary.Concat_StrStr` "Pickup location: " (`KismetStringLibrary.Conv_NameToString` (`.Name_22_DE2A3CB041D9E17CEF269189D1821695` (break `/Game/Blueprints/Inventory/Data/Struct_Store` _returnvalue_2))))) _output_get)
                (bind _result (`self.FormatItemsText`))
                (set `/Game/UI/Common/Widgets/Popups/WB_Common_DasherQuestDetailsTracker.ItemsToPickupText` (`KismetTextLibrary.Conv_StringToText` _result) (`self.DasherTrackerRef`))
                (bind _returnvalue_3 (`|GetDataTableRow` "/Game/Blueprints/Quests/Data/DT_Outposts.DT_Outposts" (`KismetStringLibrary.Conv_StringToName` (`KismetStringLibrary.Conv_IntToString` (`self.OutpostID`))))
                  (:`then`
                    (set `/Game/UI/Common/Widgets/Popups/WB_Common_DasherQuestDetailsTracker.Delivery Location Text` (`KismetTextLibrary.Conv_StringToText` (`KismetStringLibrary.Concat_StrStr` "Delivery location: " (`KismetStringLibrary.Conv_NameToString` (`.Name_5_397B80B14680E67794DFA9A74F122ADB` (break `/Game/Blueprints/Quests/Data/Struct_Outpost` _returnvalue_3))))) (`self.DasherTrackerRef`))
                    (`/Game/UI/Common/Widgets/Popups/WB_Common_DasherQuestDetailsTracker.UpdateDasherTracker` _output_get)
                    (`self.OnQuestUpdated` (`self.DasherTrackerRef`))))))))))))

(fn `MultiplyRewards`
  (params (Min :type Integer) (Max :type Integer))
  (returns (ReturnValue :type Integer))
  (bind _returnvalue (`KismetMathLibrary.RandomIntegerInRange` Min Max))
  (return (`KismetMathLibrary.FTrunc` (+ (* _returnvalue (`self.TimeMultiplier`)) (* _returnvalue (`self.DifficultyMultiplier`))))))

(fn `RemoveQuestItemsFromPlayerInventory`
  (bind _bp_inventorycomponent (`/Game/Player/Blueprints/BP_PlayerState.BP_InventoryComponent` (`self.Player State Ref`)))
  (for _array_element (`self.WantedItems`)
    (bind (_wasitemfound _fromhotbar _founditem) (`/Game/Blueprints/Inventory/AC_InventoryComponent.FindItem` _bp_inventorycomponent _array_element))
    (`/Game/Blueprints/Inventory/AC_InventoryComponent.Remove` _bp_inventorycomponent _founditem false null))
  (if _wasitemfound
    (`KismetSystemLibrary.PrintString` "Items removed")))

(fn `ResetVariables`
  (set `self.TimeElapsed` 0.0)
  (`KismetArrayLibrary.Array_Clear` (`self.WantedItems`))
  (set `self.NumberOfItems` 0)
  (set `self.PreferredStore` null)
  (set `self.PreferredStoreID` 0)
  (`KismetArrayLibrary.Array_Clear` (`self.WantedItemIDs`))
  (set `self.TargetOutpost` null)
  (set `self.TargetCustomer` null)
  (set `self.OutpostID` 0)
  (set `self.DistanceFromStoreToOutpost` 0.0)
  (set `self.DistanceFromPlayerToStore` 0.0)
  (set `self.TotalDistance_CM` 0.0)
  (set `self.EstimatedDeliveryTime` 0.0)
  (set `self.QuestDifficulty` 0)
  (set `self.Reward` (struct))
  (set `self.DifficultyMultiplier` 0.0)
  (set `self.TimeMultiplier` 0.0)
  (set `self.QuestStage` 0)
  (`KismetArrayLibrary.Array_Clear` (`self.CollectedQuestItems`))
  (set `self.hasAllQuestItems` false)
  (set `self.hasActiveQuest` false)
  (`KismetArrayLibrary.Array_Clear` (`self.Rewards`)))

(fn `SetPossibleItemIDs`
  ;[0 0 0] Get the actual data for the accessible stores
  (for _array_element (`/Game/Blueprints/Components/AC_ExperienceComponent.CurrentlyAccessibleStores` (`/Game/Player/Blueprints/BP_PlayerState.AC_ExperienceComponent` (`self.Player State Ref`)))
    (bind _returnvalue (`|GetDataTableRow` "/Game/Blueprints/Inventory/Data/DT_Stores.DT_Stores" (`KismetStringLibrary.Conv_StringToName` (`KismetStringLibrary.Conv_IntToString` _array_element)))
      (:`then`
        ;[0 0 0] Find all items within all accessible stores and add them to the possible wanted item IDs
        (for _array_element_2 (`.StoreItems_24_CD5986404855986FF0A7F9B171B9BD05` (break `/Game/Blueprints/Inventory/Data/Struct_Store` _returnvalue))
          (`KismetArrayLibrary.Array_AddUnique` (`self.PossibleWantedItemIDs`) (`.ItemID_16_631064EE4BF40380D410ECBF1096056C` (break `/Game/Blueprints/Inventory/Data/Struct_StoreItem` _array_element_2))))))))

(fn `SetReferences`
  (set `self.Player State Ref` (`/Game/Blueprints/BFL_CommonFunctions.GetPlayerStateReference`))
  (set `self.Player Character Ref` (`/Game/Blueprints/BFL_CommonFunctions.GetPlayerCharacterReference`))
  (set `self.Base Widget Ref` (`/Game/Blueprints/BFL_CommonFunctions.GetBaseWidgetRef`)))

(fn `StartQuest`
  (`self.StartQuestTimer`)
  (bind _returnvalue (`|SpawnActorFromClass` "/Game/Blueprints/Quests/BP_Waypoint.BP_Waypoint_C" (`KismetMathLibrary.MakeTransform` (`SceneComponent.K2_GetComponentLocation` (`/Game/Blueprints/Shops/BP_Store.WaypointLocation` (`self.PreferredStore`)))) "Undefined" "MultiplyWithRoot" null "" true null))
  (set `self.StoreWaypointRef` _returnvalue)
  (`/Engine/EditorBlueprintResources/StandardMacros.IncrementInt` (`self.QuestStage`)
    (:`  `
      (set `self.hasActiveQuest` true)
      (`self.OnQuestStarted`)
      (`self.OnQuestProgressed`))))

(fn `UserConstructionScript`)