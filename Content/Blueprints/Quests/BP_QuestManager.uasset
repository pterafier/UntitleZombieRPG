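; Quest manager that tracks one quest's staged objectives and completion for the player.
; On BeginPlay it loads the quest from DT_Quests and credits matching items already in the inventory.
; Objective updates fill a progress map for the current stage, granting bonus rewards and, when notifying, showing a popup and advancing the stage.
; It then rechecks completion, auto-completes through the quest log if flagged, and attempts to spawn a waypoint for tracked quests.
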(event `self.ReceiveBeginPlay`
  (`self.GetQuestDetails`)
  (`self.SetReferences`)
  (add `self.OnObjectiveHeard` (delegate `OnObjectiveHeard_Event`))
  (add `/Game/Blueprints/Quests/AC_QuestLogComponent.OnQuestCompleted` (`/Game/Player/Blueprints/BP_PlayerState.AC_QuestLogComponent` (`self.Player State Ref`)) (delegate `OnQuestCompleted_Event`))
  (add `/Game/Player/Blueprints/BP_ThirdPersonCharacter.OnObjectiveIDCalled` (`self.Player Character Ref`) (`|CreateDelegate` :!event `On Objective IDHeard`))
  ;[0 0 0] Do we already have the quest items in our inventory? if so, try to complete the quest
  (for _array_element (`.Objectives_61_82055BE24DF71941EA78CE8A46EE88C8` (break `/Game/Blueprints/Quests/Data/Struct_Quest` (`self.QuestDetails`)))
    (bind (_objectivename _objectivetype _objectiveid) (break `/Game/Blueprints/Quests/Data/Struct_Objectives` _array_element))
    (if (`|EnumEquality` _objectivetype "NewEnumerator0")
      (bind (_wasitemfound _fromhotbar _founditem) (`/Game/Blueprints/Inventory/AC_InventoryComponent.FindItem` (`/Game/Player/Blueprints/BP_PlayerState.BP_InventoryComponent` (`self.Player State Ref`)) (make `/Game/Blueprints/Inventory/Data/Struct_Item` (`KismetStringLibrary.Conv_StringToInt` _objectiveid) "None" null null "" (struct) null "NewEnumerator0" false null null false (struct :`FireRate` "NewEnumerator1" :`AmmoType` "NewEnumerator0" :`SocketRotation` (struct :`Pitch` -0.223008 :`Yaw` 82.670496 :`Roll` 14.129298)))))
      (`self.On Objective IDHeard` _objectiveid (`.Quantity_5_8D1E399245DFF28C8697A8BA5EC5307F` (break `/Game/Blueprints/Inventory/Data/Struct_InventorySlotData` _founditem)))))
  (bind _iscomplete (`self.isQuestComplete` :!label _label))
  (set `self.isCompleted` _iscomplete)
  (`self.AutoCompleteQuest`)
  (`KismetSystemLibrary.Delay` 0.2)
  (`self.TryAddWaypoint`))

(event `OnObjectiveHeard_Event`
  (`self.CheckForCompletion`)
  (`self.TryAddWaypoint`))

(event `OnQuestCompleted_Event`
  (params (QuestManager :type "/Game/Blueprints/Quests/BP_QuestManager Object Reference"))
  (`KismetArrayLibrary.Array_RemoveItem` (`/Game/Blueprints/Quests/AC_QuestLogComponent.CurrentQuests` (`/Game/Player/Blueprints/BP_PlayerState.AC_QuestLogComponent` (`self.Player State Ref`))) QuestManager))

(event `CheckForCompletion`
  ;[0 0 0] Do we already have the quest items in our inventory? if so, try to complete the quest
  (goto _label))

(event `AutoCompleteQuest`
  (bind (_questid _title _description _returntonpctext _ismainquest _objectives _completionrewards _autoaccept _autocomplete) (break `/Game/Blueprints/Quests/Data/Struct_Quest` (`self.QuestDetails`)))
  (if (and _autocomplete (`self.isCompleted`))
    (bind _ac_questlogcomponent (`/Game/Player/Blueprints/BP_PlayerState.AC_QuestLogComponent` (`self.Player State Ref`))
      (:`then`
        (`/Game/Blueprints/Quests/AC_QuestLogComponent.CompleteQuest` _ac_questlogcomponent _questid))
      (:`else`))))

(fn `GetObjectiveDataByID`
  (params (ObjectiveID :type String))
  (returns (Objective :type "/Game/Blueprints/Quests/Data/Struct_Objectives Structure"))
  (for _array_element (`.Objectives_61_82055BE24DF71941EA78CE8A46EE88C8` (break `/Game/Blueprints/Quests/Data/Struct_Quest` (`self.QuestDetails`)))
    (if (`KismetStringLibrary.EqualEqual_StrStr` (`.ObjectiveID_17_96A1B54D496DCD2428B1F3BF4B281CA9` (break `/Game/Blueprints/Quests/Data/Struct_Objectives` _array_element)) ObjectiveID)
      (return _array_element))))

(fn `GetQuestDetails`
  (bind _returnvalue (`|GetDataTableRow` "/Game/Blueprints/Quests/Data/DT_Quests.DT_Quests" (`self.QuestID`))
    (:`then`
      (set `self.QuestDetails` _returnvalue)
      (`BlueprintMapLibrary.Map_Clear` (`self.CurrentObjectiveProgress`))
      (for _array_element (`.Objectives_61_82055BE24DF71941EA78CE8A46EE88C8` (break `/Game/Blueprints/Quests/Data/Struct_Quest` (`self.QuestDetails`)))
        (`BlueprintMapLibrary.Map_Add` (`self.CurrentObjectiveProgress`) (`.ObjectiveID_17_96A1B54D496DCD2428B1F3BF4B281CA9` (break `/Game/Blueprints/Quests/Data/Struct_Objectives` _array_element)))))))

(fn `isObjectiveComplete`
  (params (ObjectiveID :type String) (`NotifyObjectiveComplete?` :type Boolean))
  (bind (_objectivename _objectivetype _objectiveid _waypointlocation _quantity) (break `/Game/Blueprints/Quests/Data/Struct_Objectives` (`self.GetObjectiveDataByID` (`local.ObjectiveID`))))
  (`/Game/Blueprints/BFL_CommonFunctions.AddRewards` (`.BonusRewards_32_94FD669B4E56C92AC417C79D51F16992` (break `/Game/Blueprints/Quests/Data/Struct_Objectives` (`self.GetObjectiveDataByID` (`local.ObjectiveID`)))) (`self.Player State Ref`))
  (if (and (>= (`BlueprintMapLibrary.Map_Find` (`self.CurrentObjectiveProgress`) (`local.ObjectiveID`)) _quantity) (`local.NotifyObjectiveComplete?`))
    (bind _returnvalue (`|CreateWidget` "/Game/UI/Common/Widgets/Popups/WB_Common_ObjectiveComplete_Popup.WB_Common_ObjectiveComplete_Popup_C" null _objectivename))
    (`UserWidget.AddToViewport` _returnvalue 0)
    (`/Engine/EditorBlueprintResources/StandardMacros.IncrementInt` (`self.CurrentStage`)
      (:`  `
        _)))
  (bind _iscomplete (`self.isQuestComplete`))
  (set `self.isCompleted` _iscomplete))

(fn `isQuestComplete`
  (returns (isComplete :type Boolean))
  (locals (Complete :type Boolean :default true))
  (for _array_element (`.Objectives_61_82055BE24DF71941EA78CE8A46EE88C8` (break `/Game/Blueprints/Quests/Data/Struct_Quest` (`self.QuestDetails`)))
    (bind (_objectivename _objectivetype _objectiveid) (break `/Game/Blueprints/Quests/Data/Struct_Objectives` _array_element))
    (if (not (>= (`BlueprintMapLibrary.Map_Find` (`self.CurrentObjectiveProgress`) _objectiveid) (`.Quantity_19_D686E91F4E52C2E3794960A53150422B` (break `/Game/Blueprints/Quests/Data/Struct_Objectives` (`self.GetObjectiveDataByID` _objectiveid)))))
      (bind _output_get (set `local.Complete` false))
      (return _output_get)))
  (return (`local.Complete`)))

(fn `On Objective IDHeard`
  (params (ObjectiveID :type String) (Value :type Integer :default 1) (`NotifyObjectiveComplete?` :type Boolean))
  (bind (_value _returnvalue) (`BlueprintMapLibrary.Map_Find` (`self.CurrentObjectiveProgress`) (`local.ObjectiveID`)))
  (bind _output (`|GetArrayItem` (`.Objectives_61_82055BE24DF71941EA78CE8A46EE88C8` (break `/Game/Blueprints/Quests/Data/Struct_Quest` (`self.QuestDetails`))) (`self.CurrentStage`)))
  (if (`KismetStringLibrary.EqualEqual_StrStr` (`.ObjectiveID_17_96A1B54D496DCD2428B1F3BF4B281CA9` (break `/Game/Blueprints/Quests/Data/Struct_Objectives` _output)) (`local.ObjectiveID`))
    (if (> (`KismetMathLibrary.SignOfInteger` Value) 0)
      (if _returnvalue
        (if (< _value (`.Quantity_19_D686E91F4E52C2E3794960A53150422B` (break `/Game/Blueprints/Quests/Data/Struct_Objectives` _output)))
          (`BlueprintMapLibrary.Map_Add` (`self.CurrentObjectiveProgress`) (`local.ObjectiveID`) (+ _value (`local.Value`)))
          (`self.isObjectiveComplete` (`local.ObjectiveID`) (`local.NotifyObjectiveComplete?`))
          (`self.OnObjectiveHeard`)
          (return))
        (else
          (return)))
      (else
        (`BlueprintMapLibrary.Map_Add` (`self.CurrentObjectiveProgress`) (`local.ObjectiveID`) (`KismetMathLibrary.Clamp` (+ (`BlueprintMapLibrary.Map_Find` (`self.CurrentObjectiveProgress`) (`local.ObjectiveID`)) (`local.Value`)) 0 1000000))
        (return)))
    (else
      (return))))

(fn `SetReferences`
  (set `self.Player State Ref` (`/Game/Blueprints/BFL_CommonFunctions.GetPlayerStateReference`))
  (set `self.Player Character Ref` (`/Game/Blueprints/BFL_CommonFunctions.GetPlayerCharacterReference`))
  (set `self.Base Widget Ref` (`/Game/Blueprints/BFL_CommonFunctions.GetBaseWidgetRef`))
  (return))

(fn `TryAddWaypoint`
  (bind (_objectivename _objectivetype _objectiveid _waypointlocation) (break `/Game/Blueprints/Quests/Data/Struct_Objectives` (`|GetArrayItem` (`.Objectives_61_82055BE24DF71941EA78CE8A46EE88C8` (break `/Game/Blueprints/Quests/Data/Struct_Quest` (`self.QuestDetails`))) (`self.CurrentStage`))))
  (bind _outactors (`GameplayStatics.GetAllActorsOfClass` "/Game/Blueprints/Quests/BP_Waypoint.BP_Waypoint_C"))
  (if (> (`KismetArrayLibrary.Array_Length` _outactors) 0)
    _
    (elif (and (!= _waypointlocation (0.0 0.0 0.0)) (`/Game/Blueprints/Quests/AC_QuestLogComponent.isQuestBeingTracked` (`/Game/Player/Blueprints/BP_PlayerState.AC_QuestLogComponent` (`self.Player State Ref`))))
      (`|SpawnActorFromClass` "/Game/Blueprints/Quests/BP_Waypoint.BP_Waypoint_C" (`KismetMathLibrary.MakeTransform` _waypointlocation) "Undefined" "MultiplyWithRoot" null "" false null)
      (else
        (bind _outactors_2 (`GameplayStatics.GetAllActorsOfClass` "/Game/Blueprints/Quests/BP_Waypoint.BP_Waypoint_C"))
        (for _array_element _outactors_2
          (`self.K2_DestroyActor` _array_element))))))

(fn `UserConstructionScript`)