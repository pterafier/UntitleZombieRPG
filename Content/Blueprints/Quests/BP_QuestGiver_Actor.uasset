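; BP_QuestGiver_Actor is a quest giver actor that automatically adds its configured quest to the player's quest log.
; One second after BeginPlay, GiveQuest adds the QuestData row through the player state's ACQuestLogComponent unless that quest is already active, ignoring its QuestID input.
; It then binds to the component's OnQuestCompleted delegate, but that handler is empty.
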(event `self.ReceiveBeginPlay`
  (bind (_questdata_datatable _questdata_rowname) (break `DataTableRowHandle` (`self.QuestData`)))
  (set `self.Player State Ref` (`/Game/Blueprints/BFL_CommonFunctions.GetPlayerStateReference`))
  (`KismetSystemLibrary.Delay` 1.0)
  (`self.GiveQuest` _questdata_rowname)
  (add `/Game/Blueprints/Quests/AC_QuestLogComponent.OnQuestCompleted` (`/Game/Player/Blueprints/BP_PlayerState.AC_QuestLogComponent` (`self.Player State Ref`)) (delegate `OnQuestCompleted_Event`)))

(event `OnQuestCompleted_Event`
  (params (QuestManager :type "/Game/Blueprints/Quests/BP_QuestManager Object Reference")))

(event `GiveQuest`
  (params (QuestID :type Name))
  (bind (_questdata_datatable _questdata_rowname) (break `DataTableRowHandle` (`self.QuestData`)))
  (bind (_questdata_datatable_2 _questdata_rowname_2) (break `DataTableRowHandle` (`self.QuestData`)))
  (if (not (`/Game/Blueprints/Quests/AC_QuestLogComponent.isQuestActive` (`/Game/Player/Blueprints/BP_PlayerState.AC_QuestLogComponent` (`self.Player State Ref`)) _questdata_rowname_2))
    (`/Game/Blueprints/Quests/AC_QuestLogComponent.AddQuest` (`/Game/Player/Blueprints/BP_PlayerState.AC_QuestLogComponent` (`self.Player State Ref`)) _questdata_rowname)))

(fn `UserConstructionScript`)