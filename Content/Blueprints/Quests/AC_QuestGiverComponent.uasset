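; Quest giver component for NPCs that offers a data table quest and handles its turn-in.
; Interact checks the player's quest log, then auto-accepts or opens the quest menu, and auto-completes or pushes a rewards popup.
; Menus go onto the base widget's menu stack, with the quest menu listing only the first objective.
; Quest giver state tracks progress, and turn-in appends an incrementing counter to the returned ObjectiveID.
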(event `self.ReceiveBeginPlay`
  (set `self.Player State Ref` (`/Game/Blueprints/BFL_CommonFunctions.GetPlayerStateReference`))
  (`KismetSystemLibrary.Delay` 0.2)
  (set `self.Base Widget Ref` (`/Game/Blueprints/BFL_CommonFunctions.GetBaseWidgetRef`)))

(fn `CheckCurrentQuestStatus`
  (bind (_questdata_datatable _questdata_rowname) (break `DataTableRowHandle` (`self.QuestData`)))
  (bind _questmanager (`/Game/Blueprints/Quests/AC_QuestLogComponent.GetQuestManager` (`/Game/Player/Blueprints/BP_PlayerState.AC_QuestLogComponent` (`self.Player State Ref`)) _questdata_rowname))
  (`/Engine/EditorBlueprintResources/StandardMacros.IsValid` _questmanager
    (:`Is Valid`
      (bind _output_get (set `self.Quest Manager` _questmanager))
      (bind (_objectivename _objectivetype _objectiveid) (break `/Game/Blueprints/Quests/Data/Struct_Objectives` (`|GetArrayItem` (`.Objectives_61_82055BE24DF71941EA78CE8A46EE88C8` (break `/Game/Blueprints/Quests/Data/Struct_Quest` (`/Game/Blueprints/Quests/BP_QuestManager.QuestDetails` _output_get))) (`/Game/Blueprints/Quests/BP_QuestManager.CurrentStage` _output_get))))
      (if (`|EnumEquality` _objectivetype "NewEnumerator6")
        (if (or (`KismetStringLibrary.EqualEqual_StrStr` _objectiveid (`self.Objective ID`)) (`KismetStringLibrary.EqualEqual_StrStr` (`KismetStringLibrary.Concat_StrStr` (`self.Objective ID`) (`KismetStringLibrary.Conv_IntToString` (`self.incrementer`))) _objectiveid) (`KismetStringLibrary.EqualEqual_StrStr` (`KismetStringLibrary.Concat_StrStr` (`self.Objective ID`) (`KismetStringLibrary.Conv_IntToString` (+ (`self.incrementer`) 1))) _objectiveid))
          (set `self.QuestGiverState` "NewEnumerator1"))))))

(fn `DisplayQuest`
  (locals (QuestDetails :type "/Game/Blueprints/Quests/Data/Struct_Quest Structure"))
  (bind (_questdata_datatable _questdata_rowname) (break `DataTableRowHandle` (`self.QuestData`)))
  (bind _base_widget_ref (`self.Base Widget Ref`))
  (bind (_questid _title _description) (break `/Game/Blueprints/Quests/Data/Struct_Quest` (`local.QuestDetails`)))
  (bind (_objectivename _objectivetype _objectiveid _waypointlocation _quantity _isoptional _bonusrewards) (break `/Game/Blueprints/Quests/Data/Struct_Objectives` (`|GetArrayItem` (`.Objectives_61_82055BE24DF71941EA78CE8A46EE88C8` (break `/Game/Blueprints/Quests/Data/Struct_Quest` (`local.QuestDetails`))))))
  (bind _returnvalue (`|GetDataTableRow` _questdata_datatable _questdata_rowname)
    (:`then`
      (set `local.QuestDetails` _returnvalue)
      (`/Game/UI/Common/Widgets/WB_Common_BaseWidget.PushWidgetToTargetStack` _base_widget_ref (`/Game/UI/Common/Widgets/WB_Common_BaseWidget.Menu_Stack` _base_widget_ref) "/Game/UI/Common/Widgets/Menus/Quests/WB_Common_QuestInteractionMenu.WB_Common_QuestInteractionMenu_C" true false)
      (bind _aswb_common_quest_interaction_menu (cast `/Game/UI/Common/Widgets/Menus/Quests/WB_Common_QuestInteractionMenu` (`/Game/UI/Common/Widgets/WB_Common_BaseWidget.PushedWidget` (`self.Base Widget Ref`))))
      (set `self.QuestMenuRef` _aswb_common_quest_interaction_menu)
      (set `TextBlock.Text` _title (`/Game/UI/Common/Widgets/Menus/Quests/WB_Common_QuestInteractionMenu.QuestTitle` (`self.QuestMenuRef`)))
      (set `TextBlock.Text` _description (`/Game/UI/Common/Widgets/Menus/Quests/WB_Common_QuestInteractionMenu.QuestDescription` (`self.QuestMenuRef`)))
      (set `/Game/UI/Common/Widgets/Menus/Quests/WB_Common_QuestInteractionMenu.QuestDetails` (`local.QuestDetails`) (`self.QuestMenuRef`))
      (bind _returnvalue_2 (`|CreateWidget` "/Game/UI/Common/Widgets/Menus/Quests/WB_Quest_ObjectiveEntry.WB_Quest_ObjectiveEntry_C" null null _objectivename _objectivetype _objectiveid _waypointlocation _quantity _isoptional _bonusrewards))
      (`PanelWidget.AddChild` (`/Game/UI/Common/Widgets/Menus/Quests/WB_Common_QuestInteractionMenu.VerticalBox_Objectives` (`self.QuestMenuRef`)) _returnvalue_2)
      (bind _asbp_npcquest_giver (cast `/Game/NPCs/QuestGivers/BP_NPCQuestGiver` (`self.GetOwner`)))
      (set `/Game/UI/Common/Widgets/Menus/Quests/WB_Common_QuestInteractionMenu.QuestGiver` _asbp_npcquest_giver (`self.QuestMenuRef`)))))

(fn `DisplayRewards`
  (bind (_questdata_datatable _questdata_rowname) (break `DataTableRowHandle` (`self.QuestData`)))
  (bind _base_widget_ref (`self.Base Widget Ref`))
  (bind _returnvalue (`|GetDataTableRow` "/Game/Blueprints/Quests/Data/DT_Quests.DT_Quests" _questdata_rowname)
    (:`then`
      (`/Game/UI/Common/Widgets/WB_Common_BaseWidget.PushWidgetToTargetStack` _base_widget_ref (`/Game/UI/Common/Widgets/WB_Common_BaseWidget.Menu_Stack` _base_widget_ref) "/Game/UI/Common/Widgets/Popups/WB_Common_QuestRewards_Popup.WB_Common_QuestRewards_Popup_C" true false)
      (bind _aswb_common_quest_rewards_popup (cast `/Game/UI/Common/Widgets/Popups/WB_Common_QuestRewards_Popup` (`/Game/UI/Common/Widgets/WB_Common_BaseWidget.PushedWidget` (`self.Base Widget Ref`))))
      (bind _output_get (set `/Game/UI/Common/Widgets/Popups/WB_Common_QuestRewards_Popup.QuestDetails` _returnvalue _aswb_common_quest_rewards_popup))
      (bind (_questid _title _description) (break `/Game/Blueprints/Quests/Data/Struct_Quest` _output_get))
      (set `TextBlock.Text` _title (`/Game/UI/Common/Widgets/Popups/WB_Common_QuestRewards_Popup.QuestTitle` _aswb_common_quest_rewards_popup))
      (set `TextBlock.Text` _description (`/Game/UI/Common/Widgets/Popups/WB_Common_QuestRewards_Popup.QuestDescription` _aswb_common_quest_rewards_popup)))))

(fn `Interact`
  (returns (ObjectiveID :type String))
  (bind (_questdata_datatable _questdata_rowname) (break `DataTableRowHandle` (`self.QuestData`)))
  (bind (_questdata_datatable_2 _questdata_rowname_2) (break `DataTableRowHandle` (`self.QuestData`)))
  (bind (_questdata_datatable_3 _questdata_rowname_3) (break `DataTableRowHandle` (`self.QuestData`)))
  (bind (_questdata_datatable_4 _questdata_rowname_4) (break `DataTableRowHandle` (`self.QuestData`)))
  (bind (_questdata_datatable_5 _questdata_rowname_5) (break `DataTableRowHandle` (`self.QuestData`)))
  (bind _ac_questlogcomponent (`/Game/Player/Blueprints/BP_PlayerState.AC_QuestLogComponent` (`self.Player State Ref`)))
  (if (and (not (`/Game/Blueprints/Quests/AC_QuestLogComponent.isQuestActive` _ac_questlogcomponent _questdata_rowname_3)) (not (`/Game/Blueprints/Quests/AC_QuestLogComponent.CheckCompletedQuests` _ac_questlogcomponent _questdata_rowname_3)))
    (bind _returnvalue (`|GetDataTableRow` "/Game/Blueprints/Quests/Data/DT_Quests.DT_Quests" _questdata_rowname)
      (:`then`
        (if (`.AutoAccept_55_C6ED3C5942F9F1FED8A373833894EB85` (break `/Game/Blueprints/Quests/Data/Struct_Quest` _returnvalue))
          (`/Game/Blueprints/Quests/AC_QuestLogComponent.AddQuest` (`/Game/Player/Blueprints/BP_PlayerState.AC_QuestLogComponent` (`self.Player State Ref`)) _questdata_rowname_5)
          (set `self.QuestGiverState` "NewEnumerator1")
          (return (`self.Objective ID`))
          (else
            (`self.DisplayQuest`)
            (return (`self.Objective ID`))))))
    (elif (`/Game/Blueprints/Quests/AC_QuestLogComponent.isQuestComplete` (`/Game/Player/Blueprints/BP_PlayerState.AC_QuestLogComponent` (`self.Player State Ref`)) _questdata_rowname_4)
      (bind _result (`/Engine/EditorBlueprintResources/StandardMacros.IncrementInt` (`self.incrementer`))
        (:`  `
          (set `self.Objective ID` (`KismetStringLibrary.Concat_StrStr` (`self.Objective ID`) (`KismetStringLibrary.Conv_IntToString` _result)))
          (bind _questmanager (`/Game/Blueprints/Quests/AC_QuestLogComponent.GetQuestManager` (`/Game/Player/Blueprints/BP_PlayerState.AC_QuestLogComponent` (`self.Player State Ref`)) _questdata_rowname_2))
          (bind (_questid _title _description _returntonpctext _ismainquest _objectives _completionrewards _autoaccept _autocomplete) (break `/Game/Blueprints/Quests/Data/Struct_Quest` (`/Game/Blueprints/Quests/BP_QuestManager.QuestDetails` _questmanager)))
          (if _autocomplete
            (set `self.QuestGiverState` "NewEnumerator2")
            (`/Game/Blueprints/Quests/AC_QuestLogComponent.CompleteQuest` (`/Game/Player/Blueprints/BP_PlayerState.AC_QuestLogComponent` (`self.Player State Ref`)) _questid)
            (return (`self.Objective ID`))
            (else
              (set `self.QuestGiverState` "NewEnumerator2")
              (`self.DisplayRewards`)
              (return (`self.Objective ID`)))))))))