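; A shop table item that the player buys with money and receives in their inventory.
; The construction script sets its mesh from the item data table using ItemID.
; Interact checks money and inventory space, deducts Price, adds the item and decrements stock, destroying the actor when none remains.
; Looking at it enables a custom depth highlight, which a per-frame looping timer clears once the character looks away.
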(event `/Game/Blueprints/Interfaces/BPI_Interact.LookAt`
  (`PrimitiveComponent.SetRenderCustomDepth` (`self.StaticMesh`) true)
  (bind _returnvalue (`KismetSystemLibrary.K2_SetTimerDelegate` (delegate `Unhighlight`) (`GameplayStatics.GetWorldDeltaSeconds`) true))
  (set `self.UnhighlightTimerHandle` _returnvalue)
  (`/Engine/EditorBlueprintResources/StandardMacros.DoOnce` false
    (:`Completed`
      (`PrimitiveComponent.SetCustomDepthStencilValue` (`self.StaticMesh`) 250))))

(event `Unhighlight`
  (if (not (== (`/Game/Player/Blueprints/BP_ThirdPersonCharacter.LookAtActor` (`self.As BP Third Person Character`)) self))
    (`PrimitiveComponent.SetRenderCustomDepth` (`self.StaticMesh`) false)
    (`KismetSystemLibrary.K2_ClearAndInvalidateTimerHandle` (`self.UnhighlightTimerHandle`))))

(fn `AddItemToPlayerInventory`
  (bind (_founditem _itemfound) (`/Game/Blueprints/BFL_CommonFunctions.GetItemFromDataTable` (`self.ItemID`)))
  (set `self.Found Item` _founditem)
  (if _itemfound
    (setmembers `/Game/Blueprints/Inventory/Data/Struct_Item` :`StructRef` (`self.Found Item`) :`PickedUpLocation` (`self.PickupLocation`))
    (`/Game/Blueprints/Inventory/AC_InventoryComponent.Add` (`/Game/Player/Blueprints/BP_PlayerState.BP_InventoryComponent` (`self.As BP Player State`)) (make `/Game/Blueprints/Inventory/Data/Struct_InventorySlotData` (`self.Found Item`) (`self.Quantity`)) false null)
    (else
      (`KismetSystemLibrary.PrintString` "Item not found in data table" true true (struct :`R` 1.0 :`G` 0.071044 :`A` 1.0) 7.0))))

(fn `Interact`
  (returns (ObjectiveID :type String))
  (if (and (>= (`/Game/Blueprints/Components/AC_BaseAttributeSet.GetMoney` (`/Game/Player/Blueprints/BP_PlayerState.AC_BaseAttributeSet` (`self.As BP Player State`))) (`self.Price`)) (`/Game/Blueprints/Inventory/AC_InventoryComponent.CheckInventorySpace` (`/Game/Player/Blueprints/BP_PlayerState.BP_InventoryComponent` (`self.As BP Player State`))) (not (`self.ItemPickedUp?`)))
    (`/Game/Blueprints/Components/AC_BaseAttributeSet.SubtractMoney` (`/Game/Player/Blueprints/BP_PlayerState.AC_BaseAttributeSet` (`self.As BP Player State`)) (`self.Price`))
    (`/Engine/EditorBlueprintResources/StandardMacros.DecrementInt` (`self.Qty`)
      (:`  `
        (if (> (`self.Qty`) 0)
          (`self.AddItemToPlayerInventory`)
          (`self.ApplyPickupEffects`)
          (`self.ItemPickedUp` (`self.ItemID`))
          (return (`KismetStringLibrary.Conv_IntToString` (`self.ItemID`)))
          (else
            (`self.AddItemToPlayerInventory`)
            (`self.SetItemPickedUp`)
            (`self.ItemPickedUp` (`self.ItemID`))
            (`self.K2_DestroyActor`)
            (return (`KismetStringLibrary.Conv_IntToString` (`self.ItemID`)))))))
    (else
      (`KismetSystemLibrary.PrintString` "You don't have enough money or your inventory is full" true true (struct :`R` 1.0 :`G` 0.06558 :`A` 1.0) 5.0))))

(fn `UserConstructionScript`
  (bind _founditem (`/Game/Blueprints/BFL_CommonFunctions.GetItemFromDataTable` (`self.ItemID`)))
  (`StaticMeshComponent.SetStaticMesh` (`self.StaticMesh`) (`.StaticMesh_58_8E4891654E1C95376986E6BC1D74FC9D` (break `/Game/Blueprints/Inventory/Data/Struct_Item` _founditem)))
  (`SceneComponent.SetWorldScale3D` (`self.StaticMesh`) (`self.MeshScale`))
  (`SceneComponent.K2_SetRelativeLocation` (`self.StaticMesh`) (`self.MeshRelativeLocation`) false false))