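; World pickup item that builds its mesh from a data table by ItemID and, on interact, adds a random quantity to the player's inventory with a pickup sound.
; Non-respawning items are destroyed; respawning ones hide, count Ultra Dynamic Sky midnight events, then reappear with a rerolled quantity.
; Look-at highlighting uses custom depth, cleared by a looping timer once the character looks away.
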(event `self.ReceiveBeginPlay`
  (`self.SetReferences`)
  (`self.SetStartingValues`)
  ;[0 0 0] Callback to UDS's Midnight dispatcher
  (add `/Game/AssetPacks/UltraDynamicSky/Blueprints/Ultra_Dynamic_Sky.Midnight` (`self.UDS`) (delegate `Midnight_Event`)))

(event `Midnight_Event`
  ;[0 0 0] Callback to UDS's Midnight dispatcher
  (if (and (`self.DoesItemRespawn?`) (`self.ItemPickedUp?`))
    (`/Engine/EditorBlueprintResources/StandardMacros.IncrementInt` (`self.DaysPassed`)
      (:`  `
        (if (> (`self.DaysPassed`) (`self.DaysBetweenRespawn`))
          (`self.RespawnItem`))))))

(event `/Game/Blueprints/Interfaces/BPI_Interact.LookAt`
  ;[0 0 0] Highlight and unhighlight based on what the player is looking at
  (`PrimitiveComponent.SetRenderCustomDepth` (`self.StaticMesh`) true)
  (bind _returnvalue (`KismetSystemLibrary.K2_SetTimerDelegate` (delegate `UnHighlightMesh`) (`GameplayStatics.GetWorldDeltaSeconds`) true))
  (set `self.UnhighlightTimerHandle` _returnvalue)
  (`/Engine/EditorBlueprintResources/StandardMacros.DoOnce` false
    (:`Completed`
      (`PrimitiveComponent.SetCustomDepthStencilValue` (`self.StaticMesh`) 250))))

(event `UnHighlightMesh`
  ;[0 0 0] Highlight and unhighlight based on what the player is looking at
  (if (not (== (`/Game/Player/Blueprints/BP_ThirdPersonCharacter.LookAtActor` (`self.As BP Third Person Character`)) self))
    (`PrimitiveComponent.SetRenderCustomDepth` (`self.StaticMesh`) false)
    (`KismetSystemLibrary.K2_ClearAndInvalidateTimerHandle` (`self.UnhighlightTimerHandle`))))

(fn `ApplyPickupEffects`
  (if (`self.OverrideDataTablePickupSound?`)
    (`GameplayStatics.PlaySound2D` (`self.PickupSoundOverride`) 1.0 1.0 0.0 null null false)
    (else
      (`GameplayStatics.PlaySound2D` (`.PickupSound_51_C375C6B54DC0C8B3537781B64EDDC133` (break `/Game/Blueprints/Inventory/Data/Struct_Item` (`self.Found Item`))) 1.0 1.0 0.0 null null false))))

(fn `Interact`
  (returns (ObjectiveID :type String))
  (if (not (`self.ItemPickedUp?`))
    (bind (_founditem _itemfound) (`/Game/Blueprints/BFL_CommonFunctions.GetItemFromDataTable` (`self.ItemID`)))
    (set `self.Found Item` _founditem)
    (if _itemfound
      (setmembers `/Game/Blueprints/Inventory/Data/Struct_Item` :`StructRef` (`self.Found Item`) :`PickedUpLocation` (`self.PickupLocation`))
      (`/Game/Blueprints/Inventory/AC_InventoryComponent.Add` (`/Game/Player/Blueprints/BP_PlayerState.BP_InventoryComponent` (`self.As BP Player State`)) (make `/Game/Blueprints/Inventory/Data/Struct_InventorySlotData` (`self.Found Item`) (`self.Quantity`)) false null)
      (`self.SetItemPickedUp`)
      (if (`self.DoesItemRespawn?`)
        (`self.ItemPickedUp` (`self.ItemID`))
        (return (`KismetStringLibrary.Conv_IntToString` (`self.ItemID`)))
        (else
          (`self.ItemPickedUp` (`self.ItemID`))
          (`self.K2_DestroyActor`)
          (return (`KismetStringLibrary.Conv_IntToString` (`self.ItemID`)))))
      (else
        (`KismetSystemLibrary.PrintString` "Item not found in data table" true true (struct :`R` 1.0 :`G` 0.071044 :`A` 1.0) 7.0)
        (return (`KismetStringLibrary.Conv_IntToString` (`self.ItemID`)))))))

(fn `RespawnItem`
  (set `self.ItemPickedUp?` false)
  (`SceneComponent.SetVisibility` (`self.StaticMesh`) true false)
  (`PrimitiveComponent.SetCollisionEnabled` (`self.StaticMesh`) "QueryOnly")
  (set `self.Quantity` (`KismetMathLibrary.RandomIntegerInRange` (`self.QuantityMin`) (`self.QuantityMax`)))
  (set `self.DaysPassed` 0))

(fn `SetItemPickedUp`
  (set `self.ItemPickedUp?` true)
  (`self.ApplyPickupEffects`)
  (`self.SetMeshInvisible`)
  (if (`self.DoesItemRespawn?`)
    (set `self.DayOfPickup` (`/Game/AssetPacks/UltraDynamicSky/Blueprints/Ultra_Dynamic_Sky.CurrentDay(Cumulative)` (`self.UDS`)))))

(fn `SetMeshInvisible`
  (`SceneComponent.SetVisibility` (`self.StaticMesh`) false false)
  (`PrimitiveComponent.SetCollisionEnabled` (`self.StaticMesh`) "NoCollision"))

(fn `SetReferences`
  (bind _uds (`/Game/AssetPacks/UltraDynamicSky/Blueprints/Functions/UltraDynamicSky_Functions.Get Ultra Dynamic Sky`))
  (set `self.UDS` _uds)
  (bind _asbp_player_state (cast `/Game/Player/Blueprints/BP_PlayerState` (`GameplayStatics.GetPlayerState` 0)))
  (set `self.As BP Player State` _asbp_player_state)
  (bind _asbp_third_person_character (cast `/Game/Player/Blueprints/BP_ThirdPersonCharacter` (`GameplayStatics.GetPlayerCharacter` 0)))
  (set `self.As BP Third Person Character` _asbp_third_person_character))

(fn `SetStartingValues`
  (set `self.Quantity` (`KismetMathLibrary.RandomIntegerInRange` (`self.QuantityMin`) (`self.QuantityMax`))))

(fn `UserConstructionScript`
  (bind _founditem (`/Game/Blueprints/BFL_CommonFunctions.GetItemFromDataTable` (`self.ItemID`)))
  (`StaticMeshComponent.SetStaticMesh` (`self.StaticMesh`) (`.StaticMesh_58_8E4891654E1C95376986E6BC1D74FC9D` (break `/Game/Blueprints/Inventory/Data/Struct_Item` _founditem)))
  (`SceneComponent.SetWorldScale3D` (`self.StaticMesh`) (`self.MeshScale`))
  (`SceneComponent.K2_SetRelativeLocation` (`self.StaticMesh`) (`self.MeshRelativeLocation`) false false))