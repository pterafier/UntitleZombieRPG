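; Inventory component that stores an owner's items in hotbar and backpack slot maps and broadcasts slot changes through dispatchers.
; Add stacks on a matching item ID, otherwise fills the hotbar before the backpack; Remove looks items up likewise.
; MoveItemToNewSlot stacks, swaps or moves items between slots and components, announcing results via an enum-selected dispatcher.
; Add and Remove also report quantity changes as quest objectives for the PlayerState-owned inventory.
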(event `self.ReceiveBeginPlay`
  (set `self.OwnerOfInventory` (`self.GetOwner`))
  (set `self.Player Character Ref` (`/Game/Blueprints/BFL_CommonFunctions.GetPlayerCharacterReference`))
  (set `self.Player State Ref` (`/Game/Blueprints/BFL_CommonFunctions.GetPlayerStateReference`)))

(fn `Add`
  (params (Item :type "/Game/Blueprints/Inventory/Data/Struct_InventorySlotData Structure") (`AddToOtherInventory?` :type Boolean) (OtherInventory :type "/Game/Blueprints/Inventory/AC_InventoryComponent Object Reference"))
  (locals (EmptyBackpackSlot :type Integer :default 0) (WasItemFound :type Boolean :default false) (FromHotbar :type Boolean :default false) (FoundItem :type "/Game/Blueprints/Inventory/Data/Struct_InventorySlotData Structure") (FoundIndex :type Integer :default 0) (LocalItem :type "/Game/Blueprints/Inventory/Data/Struct_InventorySlotData Structure"))
  (bind _emptybackpackslot (`self.FindEmptyBackpackSlot`))
  (bind (_item_item _item_quantity) (break `/Game/Blueprints/Inventory/Data/Struct_InventorySlotData` (`local.Item`)))
  (bind (_item _quantity) (break `/Game/Blueprints/Inventory/Data/Struct_InventorySlotData` (`local.LocalItem`)))
  (bind (_item_2 _quantity_2) (break `/Game/Blueprints/Inventory/Data/Struct_InventorySlotData` (`local.Item`)))
  (set `local.LocalItem` Item)
  (if (== (`self.GetOwner`) (`self.Player State Ref`))
    ;[0 0 0] Tells quest managers that an item was added to the inventory
    (`/Game/Player/Blueprints/BP_ThirdPersonCharacter.OnObjectiveIDCalled` (`self.Player Character Ref`) (`KismetStringLibrary.Conv_IntToString` (`.ID_37_2860070F4E14361ABD215881AD40851C` (break `/Game/Blueprints/Inventory/Data/Struct_Item` _item))) _quantity true))
  ;[0 0 0] Does the item already exist in one of our inventories?
  (bind (_wasitemfound _fromhotbar _founditem _foundindex) (`self.FindItem` (`.Item_2_9C6C3E8D4CDA4446392BBD8E68208A25` (break `/Game/Blueprints/Inventory/Data/Struct_InventorySlotData` (`local.Item`)))))
  (set `local.WasItemFound` _wasitemfound)
  (set `local.FromHotbar` _fromhotbar)
  (set `local.FoundItem` _founditem)
  (set `local.FoundIndex` _foundindex)
  (if (`local.WasItemFound`)
    (if (`local.FromHotbar`)
      ;[0 0 0 1 58] Stack item in hotbar
      (bind _structout (setmembers `/Game/Blueprints/Inventory/Data/Struct_InventorySlotData` :`StructRef` (`local.LocalItem`) :`Quantity` (+ (`.Quantity_5_8D1E399245DFF28C8697A8BA5EC5307F` (break `/Game/Blueprints/Inventory/Data/Struct_InventorySlotData` (`local.Item`))) (`.Quantity_5_8D1E399245DFF28C8697A8BA5EC5307F` (break `/Game/Blueprints/Inventory/Data/Struct_InventorySlotData` (`local.FoundItem`))))))
      (`BlueprintMapLibrary.Map_Add` (`self.HotbarInventory`) (`local.FoundIndex`) _structout)
      (bind (_item_3 _quantity_3) (break `/Game/Blueprints/Inventory/Data/Struct_InventorySlotData` _structout))
      (`self.ItemAddedToHotbar` _item_3 (`local.FoundIndex`) _quantity_3)
      (else
        ;[0 0 0 1 50] Stack item in backpack
        (bind _structout_2 (setmembers `/Game/Blueprints/Inventory/Data/Struct_InventorySlotData` :`StructRef` (`local.LocalItem`) :`Quantity` (+ (`.Quantity_5_8D1E399245DFF28C8697A8BA5EC5307F` (break `/Game/Blueprints/Inventory/Data/Struct_InventorySlotData` (`local.Item`))) (`.Quantity_5_8D1E399245DFF28C8697A8BA5EC5307F` (break `/Game/Blueprints/Inventory/Data/Struct_InventorySlotData` (`local.FoundItem`))))))
        (`BlueprintMapLibrary.Map_Add` (`self.BackpackInventory`) (`local.FoundIndex`) _structout_2)
        (`self.ItemAddedToBackpack` (struct) (`local.FoundIndex`))))
    (else
      (bind (_doeshotbarhavespace _firstemptyslot) (`self.CheckHotbarSpace`))
      (if _doeshotbarhavespace
        ;[0 0 0 1 50] Add item to Hotbar
        (`BlueprintMapLibrary.Map_Add` (`self.HotbarInventory`) _firstemptyslot (`local.Item`))
        (`self.ItemAddedToHotbar` _item_2 _firstemptyslot _quantity_2)
        (else
          ;[0 0 0 1 58] Add item to backpack
          (`BlueprintMapLibrary.Map_Add` (`self.BackpackInventory`) _emptybackpackslot (`local.Item`))
          (set `local.EmptyBackpackSlot` _emptybackpackslot)
          (if (`local.AddToOtherInventory?`)
            (`self.ItemAddedToOtherInventory` _item_item _item_quantity (`local.EmptyBackpackSlot`) (`local.OtherInventory`))
            (else
              (`self.ItemAddedToBackpack` (`local.Item`) (`local.EmptyBackpackSlot`)))))))))

(fn `CheckHotbarSpace`
  (returns (DoesHotbarHaveSpace :type Boolean) (FirstEmptySlot :type Integer))
  (locals (`DoesHotbarHaveSpace?` :type Boolean) (ArrayIndex :type Integer))
  (bind _values (`BlueprintMapLibrary.Map_Values` (`self.HotbarInventory`)))
  (for (_array_element _array_index) _values
    (if (`.isValid_42_1097AAAF4BC29A4DDAAB56B8A6A323F5` (break `/Game/Blueprints/Inventory/Data/Struct_Item` (`.Item_2_9C6C3E8D4CDA4446392BBD8E68208A25` (break `/Game/Blueprints/Inventory/Data/Struct_InventorySlotData` _array_element))))
      (set `local.DoesHotbarHaveSpace?` false)
      (else
        (set `local.DoesHotbarHaveSpace?` true)
        (set `local.ArrayIndex` _array_index)
        (break))))
  (return (`local.DoesHotbarHaveSpace?`) (`local.ArrayIndex`)))

(fn `CheckInventorySpace`
  (returns (hasSpace :type Boolean))
  (locals (`DoesInventoryHaveSpace?` :type Boolean) (ArrayIndex :type Integer))
  (bind _values (`BlueprintMapLibrary.Map_Values` (`self.HotbarInventory`)))
  (for (_array_element _array_index) _values
    (if (`.isValid_42_1097AAAF4BC29A4DDAAB56B8A6A323F5` (break `/Game/Blueprints/Inventory/Data/Struct_Item` (`.Item_2_9C6C3E8D4CDA4446392BBD8E68208A25` (break `/Game/Blueprints/Inventory/Data/Struct_InventorySlotData` _array_element))))
      (set `local.DoesInventoryHaveSpace?` false)
      (else
        (set `local.DoesInventoryHaveSpace?` true)
        (set `local.ArrayIndex` _array_index)
        (break))))
  (if (`local.DoesInventoryHaveSpace?`)
    (return true)
    (else
      (bind _values_2 (`BlueprintMapLibrary.Map_Values` (`self.BackpackInventory`)))
      (for (_array_element_2 _array_index_2) _values_2
        (if (`.isValid_42_1097AAAF4BC29A4DDAAB56B8A6A323F5` (break `/Game/Blueprints/Inventory/Data/Struct_Item` (`.Item_2_9C6C3E8D4CDA4446392BBD8E68208A25` (break `/Game/Blueprints/Inventory/Data/Struct_InventorySlotData` _array_element_2))))
          (set `local.DoesInventoryHaveSpace?` false)
          (else
            (set `local.DoesInventoryHaveSpace?` true)
            (set `local.ArrayIndex` _array_index_2)
            (break))))
      (return (`local.DoesInventoryHaveSpace?`)))))

(fn `FindEmptyBackpackSlot`
  (returns (EmptyBackpackSlot :type Integer))
  (locals (EmptySlot :type Integer))
  (bind _values (`BlueprintMapLibrary.Map_Values` (`self.BackpackInventory`)))
  (for (_array_element _array_index) _values
    (if (not (`.isValid_42_1097AAAF4BC29A4DDAAB56B8A6A323F5` (break `/Game/Blueprints/Inventory/Data/Struct_Item` (`.Item_2_9C6C3E8D4CDA4446392BBD8E68208A25` (break `/Game/Blueprints/Inventory/Data/Struct_InventorySlotData` _array_element)))))
      (set `local.EmptySlot` _array_index)
      (break)))
  (return (`local.EmptySlot`)))

(fn `FindEmptyHotbarSlot`
  (returns (EmptyHotbarSlot :type Integer))
  (locals (EmptySlot :type Integer :default 0))
  (bind _values (`BlueprintMapLibrary.Map_Values` (`self.HotbarInventory`)))
  (for (_array_element _array_index) _values
    (if (not (`.isValid_42_1097AAAF4BC29A4DDAAB56B8A6A323F5` (break `/Game/Blueprints/Inventory/Data/Struct_Item` (`.Item_2_9C6C3E8D4CDA4446392BBD8E68208A25` (break `/Game/Blueprints/Inventory/Data/Struct_InventorySlotData` _array_element)))))
      (set `local.EmptySlot` _array_index)
      (break)))
  (return (`local.EmptySlot`)))

(fn `FindItem`
  (params (Item :type "/Game/Blueprints/Inventory/Data/Struct_Item Structure"))
  (returns (WasItemFound :type Boolean) (FromHotbar :type Boolean) (FoundItem :type "/Game/Blueprints/Inventory/Data/Struct_InventorySlotData Structure") (FoundIndex :type Integer))
  (locals (FoundItem_Local :type "/Game/Blueprints/Inventory/Data/Struct_InventorySlotData Structure") (FoundIndex_Local :type Integer) (`WasItemInHotbar?_Local` :type Boolean) (FoundQuantity_Local :type Integer) (`WasItemFound?_Local` :type Boolean))
  (bind _values (`BlueprintMapLibrary.Map_Values` (`self.HotbarInventory`)))
  (bind (_founditem _wasitemfound_ _foundindex) (`self.FindItemInSpecificInventory` _values (`local.Item`)))
  (set `local.FoundItem_Local` _founditem)
  (set `local.WasItemFound?_Local` _wasitemfound_)
  (set `local.FoundIndex_Local` _foundindex)
  (if _wasitemfound_
    (return (`local.WasItemFound?_Local`) true (`local.FoundItem_Local`) (`local.FoundIndex_Local`))
    (else
      (bind _values_2 (`BlueprintMapLibrary.Map_Values` (`self.BackpackInventory`)))
      (bind (_founditem_2 _wasitemfound__2 _foundindex_2) (`self.FindItemInSpecificInventory` _values_2 (`local.Item`)))
      (set `local.FoundItem_Local` _founditem_2)
      (set `local.FoundIndex_Local` _foundindex_2)
      (return _wasitemfound__2 false (`local.FoundItem_Local`) (`local.FoundIndex_Local`)))))

(fn `FindItemInSpecificInventory`
  (params (InventoryValues :type "Array of /Game/Blueprints/Inventory/Data/Struct_InventorySlotData Structure") (Item :type "/Game/Blueprints/Inventory/Data/Struct_Item Structure"))
  (returns (FoundItem :type "/Game/Blueprints/Inventory/Data/Struct_InventorySlotData Structure") (`WasItemFound?` :type Boolean) (FoundIndex :type Integer))
  (locals (FoundQuantity_Local :type Integer) (`WasItemFound?_Local` :type Boolean) (`WasItemInHotbar?_Local` :type Boolean) (FoundIndex_Local :type Integer) (FoundItem_Local :type "/Game/Blueprints/Inventory/Data/Struct_InventorySlotData Structure"))
  (for (_array_element _array_index) InventoryValues
    (bind (_item _quantity) (break `/Game/Blueprints/Inventory/Data/Struct_InventorySlotData` _array_element))
    (if (== (`.ID_37_2860070F4E14361ABD215881AD40851C` (break `/Game/Blueprints/Inventory/Data/Struct_Item` _item)) (`.ID_37_2860070F4E14361ABD215881AD40851C` (break `/Game/Blueprints/Inventory/Data/Struct_Item` (`local.Item`))))
      (set `local.FoundItem_Local` _array_element)
      (set `local.FoundIndex_Local` _array_index)
      (set `local.WasItemFound?_Local` true)
      (set `local.FoundQuantity_Local` _quantity)
      (break)
      (else
        (set `local.WasItemFound?_Local` false))))
  (return (`local.FoundItem_Local`) (`local.WasItemFound?_Local`) (`local.FoundIndex_Local`)))

(fn `FindQuestItemByObjectiveID`
  (params (Item :type "/Game/Blueprints/Inventory/Data/Struct_Item Structure"))
  (returns (WasItemFound :type Boolean) (FromHotbar :type Boolean) (FoundItem :type "/Game/Blueprints/Inventory/Data/Struct_InventorySlotData Structure") (FoundIndex :type Integer))
  (locals (FoundQuestItem_Local :type "/Game/Blueprints/Inventory/Data/Struct_InventorySlotData Structure") (FoundQuestIndex_Local :type Integer) (`WasQuestItemInHotbar?_Local` :type Boolean) (FoundQuestQuantity_Local :type Integer) (`WasQuestItemFound?_Local` :type Boolean) (MatchingQuestItems :type "Array of /Game/Blueprints/Inventory/Data/Struct_Item Structure"))
  (bind _values (`BlueprintMapLibrary.Map_Values` (`self.HotbarInventory`)))
  (bind (_founditem _wasitemfound_ _foundindex) (`self.FindItemInSpecificInventory` _values (`local.Item`)))
  (set `local.FoundQuestItem_Local` _founditem)
  (set `local.WasQuestItemFound?_Local` _wasitemfound_)
  (set `local.FoundQuestIndex_Local` _foundindex)
  (if _wasitemfound_
    (return (`local.WasQuestItemFound?_Local`) true (`local.FoundQuestItem_Local`) (`local.FoundQuestIndex_Local`))
    (else
      (bind _values_2 (`BlueprintMapLibrary.Map_Values` (`self.BackpackInventory`)))
      (bind (_founditem_2 _wasitemfound__2 _foundindex_2) (`self.FindItemInSpecificInventory` _values_2 (`local.Item`)))
      (set `local.FoundQuestItem_Local` _founditem_2)
      (set `local.FoundQuestIndex_Local` _foundindex_2)
      (return _wasitemfound__2 false (`local.FoundQuestItem_Local`) (`local.FoundQuestIndex_Local`)))))

(fn `MoveItemToNewSlot`
  (params (FromSlot :type Integer) (ToSlot :type Integer) (ToInventory :type "Map of Integer to /Game/Blueprints/Inventory/Data/Struct_InventorySlotData Structure") (FromInventory :type "Map of Integer to /Game/Blueprints/Inventory/Data/Struct_InventorySlotData Structure") (FromInventoryComponent :type "/Game/Blueprints/Inventory/AC_InventoryComponent Object Reference") (ToInventoryComponent :type "/Game/Blueprints/Inventory/AC_InventoryComponent Object Reference") (TO_Delegate :type "/Game/Blueprints/Inventory/Data/Enum_IconDelegates Enum" :default "NewEnumerator0") (FROM_Delegate :type "/Game/Blueprints/Inventory/Data/Enum_IconDelegates Enum" :default "NewEnumerator0"))
  (returns (ItemFrom_FROM_Slot :type "/Game/Blueprints/Inventory/Data/Struct_InventorySlotData Structure") (ItemFrom_TO_Slot :type "/Game/Blueprints/Inventory/Data/Struct_InventorySlotData Structure"))
  (locals (ItemInToSlot :type Boolean) (`SlotsInSameInventory?` :type Boolean) (EnumSelection :type "/Game/Blueprints/Inventory/Data/Enum_IconDelegates Enum" :default "NewEnumerator0") (SavedItemInToSlot :type "/Game/Blueprints/Inventory/Data/Struct_InventorySlotData Structure") (SavedItemInFromSlot :type "/Game/Blueprints/Inventory/Data/Struct_InventorySlotData Structure") (ToSlotItemID :type Integer) (FromSlotItemID :type Integer))
  (bind _savediteminfromslot (`local.SavedItemInFromSlot`))
  (bind _value (`BlueprintMapLibrary.Map_Find` (`local.ToInventory`) (`local.ToSlot`)))
  (bind _value_2 (`BlueprintMapLibrary.Map_Find` (`local.FromInventory`) (`local.FromSlot`)))
  (bind (_id _name _icon _staticmesh _description _buyselldata _actor _equip _isvalid) (break `/Game/Blueprints/Inventory/Data/Struct_Item` (`.Item_2_9C6C3E8D4CDA4446392BBD8E68208A25` (break `/Game/Blueprints/Inventory/Data/Struct_InventorySlotData` _value))))
  ;[0 0 0] If the player picks up the item and drops it in the same slot, do nothing
  (if (and (== (`local.ToSlot`) (`local.FromSlot`)) (== (`local.FromInventoryComponent`) (`local.ToInventoryComponent`)) (== (`BlueprintMapLibrary.Map_Length` (`local.ToInventory`)) (`BlueprintMapLibrary.Map_Length` (`local.FromInventory`))))
    ;[0 0 0] Return exactly what was input
    (return (`BlueprintMapLibrary.Map_Find` (`local.FromInventory`) (`local.FromSlot`)) (`BlueprintMapLibrary.Map_Find` (`local.ToInventory`) (`local.ToSlot`)))
    (else
      (`|ExecutionSequence`
        (:`then_0`
          ;[0 0 0] Set variables based on items in to and from slots
          (set `local.ToSlotItemID` _id)
          (set `local.SavedItemInToSlot` _value)
          (set `local.ItemInToSlot` _isvalid))
        (:`then_1`
          (set `local.FromSlotItemID` (`.ID_37_2860070F4E14361ABD215881AD40851C` (break `/Game/Blueprints/Inventory/Data/Struct_Item` (`.Item_2_9C6C3E8D4CDA4446392BBD8E68208A25` (break `/Game/Blueprints/Inventory/Data/Struct_InventorySlotData` _value_2)))))
          (set `local.SavedItemInFromSlot` _value_2)
          ;[0 0 0] If "to" slot has an item:
          (if (`local.ItemInToSlot`)
            ;[0 0 0] Do the items have the same ID? Should we stack?
            (if (== (`local.ToSlotItemID`) (`local.FromSlotItemID`))
              ;[0 0 0] Stack item
              (`|ExecutionSequence`
                (:`then_0`
                  ;;[0.05 0.05 0.05] Add the "from" and "to" slot's quantities together, and add them back into the "to" slot (stack the item). Call the generic dispatcher to notify MainOverlay of change
                  (bind _structout (setmembers `/Game/Blueprints/Inventory/Data/Struct_InventorySlotData` :`StructRef` _savediteminfromslot :`Quantity` (+ (`.Quantity_5_8D1E399245DFF28C8697A8BA5EC5307F` (break `/Game/Blueprints/Inventory/Data/Struct_InventorySlotData` _savediteminfromslot)) (`.Quantity_5_8D1E399245DFF28C8697A8BA5EC5307F` (break `/Game/Blueprints/Inventory/Data/Struct_InventorySlotData` (`local.SavedItemInToSlot`))))))
                  (`self.SelectAndFireDelegate` (`local.TO_Delegate`) _structout (`local.ToSlot`) (`local.ToInventoryComponent`)))
                (:`then_1`
                  ;;[0.05 0.05 0.05] Replace the item in the "from" slot with an empty item. Call the dispatcher to change icons.
                  (`self.SelectAndFireDelegate` (`local.FROM_Delegate`) (make `/Game/Blueprints/Inventory/Data/Struct_InventorySlotData` (`self.EmptyItem`)) (`local.FromSlot`) (`local.FromInventoryComponent`))
                  (return _structout (make `/Game/Blueprints/Inventory/Data/Struct_InventorySlotData` (`self.EmptyItem`)))))
              (else
                ;[0 0 0] Swap Items
                (`|ExecutionSequence`
                  (:`then_0`
                    ;;[0.05 0.05 0.05] Add the item from the "from" slot to the "to" slot
                    (`self.SelectAndFireDelegate` (`local.TO_Delegate`) (`local.SavedItemInFromSlot`) (`local.ToSlot`) (`local.ToInventoryComponent`)))
                  (:`then_1`
                    ;;[0.05 0.05 0.05] Fires "Added to" delegates instead of "Removed from" so the icons aren't cleared
                    (switch `/Game/Blueprints/Inventory/Data/Enum_IconDelegates` (`local.FROM_Delegate`)
                      (:`NewEnumerator3`
                        (set `local.EnumSelection` "NewEnumerator0"))
                      (:`NewEnumerator4`
                        (set `local.EnumSelection` "NewEnumerator1"))
                      (:`NewEnumerator5`
                        (set `local.EnumSelection` "NewEnumerator2")))
                    (`self.SelectAndFireDelegate` (`local.EnumSelection`) (`local.SavedItemInToSlot`) (`local.FromSlot`) (`local.FromInventoryComponent`))
                    (return (`local.SavedItemInFromSlot`) (`local.SavedItemInToSlot`))))))
            (else
              (`|ExecutionSequence`
                (:`then_0`
                  ;[0 0 0] Add the item from the "from" slot to the "to" slot
                  (`self.SelectAndFireDelegate` (`local.TO_Delegate`) (`local.SavedItemInFromSlot`) (`local.ToSlot`) (`local.ToInventoryComponent`)))
                (:`then_1`
                  ;[0 0 0] Replace the item in the "from" slot with an empty item
                  (`self.SelectAndFireDelegate` (`local.FROM_Delegate`) (`local.SavedItemInFromSlot`) (`local.FromSlot`) (`local.FromInventoryComponent`))
                  (return (`local.SavedItemInFromSlot`) (make `/Game/Blueprints/Inventory/Data/Struct_InventorySlotData` (`self.EmptyItem`))))))))))))

(fn `Remove`
  (params (Item :type "/Game/Blueprints/Inventory/Data/Struct_InventorySlotData Structure") (`RemoveFromOtherInventory?` :type Boolean) (OtherInventory :type "/Game/Blueprints/Inventory/AC_InventoryComponent Object Reference"))
  (locals (EmptyBackpackSlot :type Integer :default 0) (WasItemFound :type Boolean :default false) (FromHotbar :type Boolean :default false) (FoundItem :type "/Game/Blueprints/Inventory/Data/Struct_InventorySlotData Structure") (FoundIndex :type Integer :default 0))
  (bind (_item _quantity) (break `/Game/Blueprints/Inventory/Data/Struct_InventorySlotData` (`local.Item`)))
  ;[0 0 0] Does the item already exist in one of our inventories?
  (bind (_wasitemfound _fromhotbar _founditem _foundindex) (`self.FindItem` (`.Item_2_9C6C3E8D4CDA4446392BBD8E68208A25` (break `/Game/Blueprints/Inventory/Data/Struct_InventorySlotData` (`local.Item`)))))
  (set `local.WasItemFound` _wasitemfound)
  (set `local.FromHotbar` _fromhotbar)
  (set `local.FoundItem` _founditem)
  (set `local.FoundIndex` _foundindex)
  (if (`local.WasItemFound`)
    (if (== (`self.OwnerOfInventory`) (`self.Player State Ref`))
      (`/Game/Player/Blueprints/BP_ThirdPersonCharacter.OnObjectiveIDCalled` (`self.Player Character Ref`) (`KismetStringLibrary.Conv_IntToString` (`.ID_37_2860070F4E14361ABD215881AD40851C` (break `/Game/Blueprints/Inventory/Data/Struct_Item` _item))) (* _quantity -1) true))
    (if (`local.FromHotbar`)
      ;[0 0 0] Do we have less items than we're trying to remove?
      (if (<= (`.Quantity_5_8D1E399245DFF28C8697A8BA5EC5307F` (break `/Game/Blueprints/Inventory/Data/Struct_InventorySlotData` (`local.FoundItem`))) (`.Quantity_5_8D1E399245DFF28C8697A8BA5EC5307F` (break `/Game/Blueprints/Inventory/Data/Struct_InventorySlotData` (`local.Item`))))
        ;[0 0 0] Replace the slot with an empty item
        (`BlueprintMapLibrary.Map_Add` (`self.HotbarInventory`) (`local.FoundIndex`) (make `/Game/Blueprints/Inventory/Data/Struct_InventorySlotData` (`self.EmptyItem`)))
        (`self.ItemRemovedFromHotbar` (struct) (`local.FoundIndex`))
        (else
          ;[0 0 0 1 58] Stack item in hotbar
          (bind _structout (setmembers `/Game/Blueprints/Inventory/Data/Struct_InventorySlotData` :`StructRef` (`local.FoundItem`) :`Quantity` (`KismetMathLibrary.Clamp` (- (`.Quantity_5_8D1E399245DFF28C8697A8BA5EC5307F` (break `/Game/Blueprints/Inventory/Data/Struct_InventorySlotData` (`local.FoundItem`))) (`.Quantity_5_8D1E399245DFF28C8697A8BA5EC5307F` (break `/Game/Blueprints/Inventory/Data/Struct_InventorySlotData` (`local.Item`)))) 0 1000000000)))
          (`BlueprintMapLibrary.Map_Add` (`self.HotbarInventory`) (`local.FoundIndex`) _structout)
          (bind (_item_2 _quantity_2) (break `/Game/Blueprints/Inventory/Data/Struct_InventorySlotData` _structout))
          (`self.ItemAddedToHotbar` _item_2 (`local.FoundIndex`) _quantity_2)))
      (else
        ;[0 0 0] Do we have less items than we're trying to remove?
        (if (<= (`.Quantity_5_8D1E399245DFF28C8697A8BA5EC5307F` (break `/Game/Blueprints/Inventory/Data/Struct_InventorySlotData` (`local.FoundItem`))) (`.Quantity_5_8D1E399245DFF28C8697A8BA5EC5307F` (break `/Game/Blueprints/Inventory/Data/Struct_InventorySlotData` (`local.Item`))))
          ;[0 0 0] Replace the slot with an empty item
          (`BlueprintMapLibrary.Map_Add` (`self.BackpackInventory`) (`local.FoundIndex`) (make `/Game/Blueprints/Inventory/Data/Struct_InventorySlotData` (`self.EmptyItem`)))
          (`self.ItemRemovedFromBackpack` (struct) (`local.FoundIndex`))
          (else
            ;[0 0 0 1 50] Stack item in backpack
            (bind _structout_2 (setmembers `/Game/Blueprints/Inventory/Data/Struct_InventorySlotData` :`StructRef` (`local.FoundItem`) :`Quantity` (+ (`.Quantity_5_8D1E399245DFF28C8697A8BA5EC5307F` (break `/Game/Blueprints/Inventory/Data/Struct_InventorySlotData` (`local.Item`))) (`.Quantity_5_8D1E399245DFF28C8697A8BA5EC5307F` (break `/Game/Blueprints/Inventory/Data/Struct_InventorySlotData` (`local.FoundItem`))))))
            (`BlueprintMapLibrary.Map_Add` (`self.BackpackInventory`) (`local.FoundIndex`) _structout_2)
            (`self.ItemAddedToBackpack` _structout_2 (`local.FoundIndex`))))))
    (else
      (`KismetSystemLibrary.PrintString` "You're trying to remove an item that doesn't exist in this inventory component"))))

(fn `RemoveAllItemsFromBackpack`
  (`BlueprintMapLibrary.Map_Clear` (`self.BackpackInventory`))
  (for _index (range 10)
    (`BlueprintMapLibrary.Map_Add` (`self.BackpackInventory`) _index (make `/Game/Blueprints/Inventory/Data/Struct_InventorySlotData` (`self.EmptyItem`)))
    (`self.ItemRemovedFromOtherInventory` _index)))

(fn `SelectAndFireDelegate`
  (params (Selection :type "/Game/Blueprints/Inventory/Data/Enum_IconDelegates Enum" :default "NewEnumerator0") (ItemSlot :type "/Game/Blueprints/Inventory/Data/Struct_InventorySlotData Structure") (SlotIndex :type Integer) (OtherInventory :type "/Game/Blueprints/Inventory/AC_InventoryComponent Object Reference"))
  (bind (_itemslot_item _itemslot_quantity) (break `/Game/Blueprints/Inventory/Data/Struct_InventorySlotData` (`local.ItemSlot`)))
  (bind (_itemslot_item_2 _itemslot_quantity_2) (break `/Game/Blueprints/Inventory/Data/Struct_InventorySlotData` (`local.ItemSlot`)))
  (bind (_itemslot_item_3 _itemslot_quantity_3) (break `/Game/Blueprints/Inventory/Data/Struct_InventorySlotData` (`local.ItemSlot`)))
  (switch `/Game/Blueprints/Inventory/Data/Enum_IconDelegates` Selection
    (:`NewEnumerator0`
      (`self.ItemAddedToBackpack` (`local.ItemSlot`) (`local.SlotIndex`)))
    (:`NewEnumerator1`
      (`self.ItemAddedToHotbar` _itemslot_item_3 (`local.SlotIndex`) _itemslot_quantity_3))
    (:`NewEnumerator2`
      (`self.ItemAddedToOtherInventory` _itemslot_item_2 _itemslot_quantity_2 (`local.SlotIndex`) (`local.OtherInventory`)))
    (:`NewEnumerator3`
      (`self.ItemRemovedFromBackpack` (struct) (`local.SlotIndex`)))
    (:`NewEnumerator4`
      (`self.ItemRemovedFromHotbar` (struct) (`local.SlotIndex`)))
    (:`NewEnumerator5`
      (`self.ItemRemovedFromOtherInventory` (`local.SlotIndex`) _itemslot_item _itemslot_quantity))))